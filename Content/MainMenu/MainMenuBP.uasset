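; Main menu Blueprint that holds a camera and four pages of static mesh components.
; The Rotate event instantly yaws the camera in 90-degree steps by the given page count, with a Left flag choosing the direction.
; The construction script groups the mesh components into four page arrays of three each, which this graph does not otherwise read.
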(event Custom|Rotate
  (params (Left :type Boolean) (Pages :type Integer))
  (bind _camera (Variables|Default|GetCamera))
  (if Left
    (Transformation|AddRelativeRotation _camera (Math|Rotator|MakeRotator 0.0 0.0 (* Pages -9e+01)) false false)
    (else
      (Transformation|AddRelativeRotation _camera (Math|Rotator|MakeRotator 0.0 0.0 (* Pages 9e+01)) false false))))

(fn ConstructionScript
  (Variables|Default|SetPagina1 (Utilities|Array|MakeArray (Variables|Default|GetStaticMesh) (Variables|Default|GetStaticMesh1) (Variables|Default|GetCube)))
  (Variables|Default|SetPagina2 (Utilities|Array|MakeArray (Variables|Default|GetStaticMesh3) (Variables|Default|GetStaticMesh4) (Variables|Default|GetStaticMesh2)))
  (Variables|Default|SetPagina3 (Utilities|Array|MakeArray (Variables|Default|GetStaticMesh6) (Variables|Default|GetStaticMesh7) (Variables|Default|GetStaticMesh5)))
  (Variables|Default|SetPagina4 (Utilities|Array|MakeArray (Variables|Default|GetStaticMesh9) (Variables|Default|GetStaticMesh10) (Variables|Default|GetStaticMesh8))))