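; Configurable level-building module whose construction script assembles a straight, curved or four-exit section from static meshes, chosen by TipoModulo.
; Straight modules use per-side options and helper functions for walls, grids, tubes, panels, skirtings and columns, with checks against combining closed column panels with on-floor tubes.
; Curved and four-exit modules hide the trap child actors.
; SetTraps runs an empty sequence, leaving its trap mesh and enabling logic disconnected.
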(fn ConstructionScript
  (bind _dritto_roof (Variables|Default|GetDRITTO_Roof))
  (bind _dritto_wallleft (Variables|Default|GetDRITTO_WallLeft))
  (bind _curvo_rollup (Variables|Default|GetCURVO_RollUp))
  (bind _dritto_wallright (Variables|Default|GetDRITTO_WallRight))
  (bind _dritto_uppersidegridleft (Variables|Default|GetDRITTO_UpperSideGridLeft))
  (bind _dritto_uppersidegridright (Variables|Default|GetDRITTO_UpperSideGridRight))
  (switch Utilities|FlowControl|Switch|SwitchonENUM_DRITTO_TipoModuli (Variables|Default|GetTipoModulo)
    (:NewEnumerator0
      ;[1 1 1] Gestione Tipo Modulo Dritto
      (Utilities|FlowControl|Sequence
        (:then_0
          (switch Utilities|FlowControl|Switch|SwitchonENUM_DRITTO_Roof (Variables|Struttura|GetDRITTO_TipoRoof)
            (:NewEnumerator0
              (Components|StaticMesh|SetStaticMesh _dritto_roof "/Game/Maps/Moduli/Mesh/Dritto/G_Straight_Roof_Libero_002.G_Straight_Roof_Libero_002"))
            (:NewEnumerator1
              (Components|StaticMesh|SetStaticMesh _dritto_roof "/Game/Maps/Moduli/Mesh/Dritto/G_Straight_Roof_WithGrid_002.G_Straight_Roof_WithGrid_002")
              (Components|StaticMesh|SetStaticMesh (Variables|Default|GetDRITTO_RoofGrid) "/Game/Maps/Moduli/Mesh/Dritto/G_Straight_Roof_Grid_002.G_Straight_Roof_Grid_002")))
          (Components|StaticMesh|SetStaticMesh (Variables|Default|GetDRITTO_Floor) "/Game/Maps/Moduli/Mesh/Dritto/G_Straight_Floor_001.G_Straight_Floor_001"))
        (:then_1
          (switch Utilities|FlowControl|Switch|SwitchonENUM_DRITTO_Muri (Variables|Struttura|GetDRITTO_TipoMuroLeft)
            (:NewEnumerator4
              (Components|StaticMesh|SetStaticMesh _dritto_wallleft "/Game/Maps/Moduli/Mesh/Dritto/G_Straight_Wall_Libero_001.G_Straight_Wall_Libero_001"))
            (:NewEnumerator5
              (Components|StaticMesh|SetStaticMesh _dritto_wallleft "/Game/Maps/Moduli/Mesh/Dritto/G_Straight_Wall_With_Traps_002.G_Straight_Wall_With_Traps_002")))
          (switch Utilities|FlowControl|Switch|SwitchonENUM_DRITTO_Muri (Variables|Struttura|GetDRITTO_TipoMuroRight)
            (:NewEnumerator4
              (Components|StaticMesh|SetStaticMesh _dritto_wallright "/Game/Maps/Moduli/Mesh/Dritto/G_Straight_Wall_Libero_001.G_Straight_Wall_Libero_001"))
            (:NewEnumerator5
              (Components|StaticMesh|SetStaticMesh _dritto_wallright "/Game/Maps/Moduli/Mesh/Dritto/G_Straight_Wall_With_Traps_002.G_Straight_Wall_With_Traps_002"))))
        (:then_2
          (CallFunction|SetTraps))
        (:then_3
          (CallFunction|SetWallBases))
        (:then_4
          (CallFunction|SetLowerSideTubesPannels))
        (:then_5
          (CallFunction|SetSkirtings))
        (:then_6
          (CallFunction|SetColumnSlots))
        (:then_7
          (Components|StaticMesh|SetStaticMesh (Variables|Default|GetDRITTO_GrataAngleTrapLeft) "/Game/Maps/Moduli/Mesh/Dritto/G_Straight_Oblique_Trap_Grid_001.G_Straight_Oblique_Trap_Grid_001")
          (Components|StaticMesh|SetStaticMesh (Variables|Default|GetDRITTO_GrataAngleTrapRight) "/Game/Maps/Moduli/Mesh/Dritto/G_Straight_Oblique_Trap_Grid_001.G_Straight_Oblique_Trap_Grid_001"))
        (:then_8
          (switch Utilities|FlowControl|Switch|SwitchonENUM_DRITTO_SideGrid (Variables|Struttura|GetDRITTO_TipoSideGridLeft)
            (:NewEnumerator0
              (Components|StaticMesh|SetStaticMesh _dritto_uppersidegridleft "/Game/Maps/Moduli/Mesh/Dritto/G_Straight_Side_Grid_Grid_001.G_Straight_Side_Grid_Grid_001"))
            (:NewEnumerator1
              (Components|StaticMesh|SetStaticMesh _dritto_uppersidegridleft "/Game/Maps/Moduli/Mesh/Dritto/G_Straight_Side_Grid_Broken_001.G_Straight_Side_Grid_Broken_001"))
            (:NewEnumerator2
              (Components|StaticMesh|SetStaticMesh _dritto_uppersidegridleft "/Game/Maps/Moduli/Mesh/Dritto/G_Straight_Side_Grid_Tubi_001.G_Straight_Side_Grid_Tubi_001")))
          (switch Utilities|FlowControl|Switch|SwitchonENUM_DRITTO_SideGrid (Variables|Struttura|GetDRITTO_TipoSideGridRight)
            (:NewEnumerator0
              (Components|StaticMesh|SetStaticMesh _dritto_uppersidegridright "/Game/Maps/Moduli/Mesh/Dritto/G_Straight_Side_Grid_Grid_001.G_Straight_Side_Grid_Grid_001"))
            (:NewEnumerator1
              (Components|StaticMesh|SetStaticMesh _dritto_uppersidegridright "/Game/Maps/Moduli/Mesh/Dritto/G_Straight_Side_Grid_Broken_001.G_Straight_Side_Grid_Broken_001"))
            (:NewEnumerator2
              (Components|StaticMesh|SetStaticMesh _dritto_uppersidegridright "/Game/Maps/Moduli/Mesh/Dritto/G_Straight_Side_Grid_Tubi_001.G_Straight_Side_Grid_Tubi_001"))))))
    (:NewEnumerator1
      ;[1 1 1] Modulo Curvo
      (CallFunction|HideTraps false)
      (Utilities|FlowControl|Sequence
        (:then_0
          (Components|StaticMesh|SetStaticMesh (Variables|Default|GetCURVO_Wall) "/Game/Maps/Moduli/Mesh/Curvo/G_Curve_Wall.G_Curve_Wall")
          (Components|StaticMesh|SetStaticMesh (Variables|Default|GetCURVO_Roof) "/Game/Maps/Moduli/Mesh/Curvo/G_Curve_Roof.G_Curve_Roof")
          (Components|StaticMesh|SetStaticMesh (Variables|Default|GetCURVO_Floor) "/Game/Maps/Moduli/Mesh/Curvo/G_Curve_Floor.G_Curve_Floor")
          (Components|StaticMesh|SetStaticMesh (Variables|Default|GetCURVO_Column) "/Game/Maps/Moduli/Mesh/Curvo/G_Curve_Column.G_Curve_Column")
          (Components|StaticMesh|SetStaticMesh (Variables|Default|GetCURVE_Tubes) "/Game/Maps/Moduli/Mesh/Curvo/G_Curve_Tubes.G_Curve_Tubes"))
        (:then_1
          (Components|StaticMesh|SetStaticMesh _curvo_rollup "/Game/Maps/Moduli/Mesh/Curvo/G_Curve_RollUp.G_Curve_RollUp")
          (switch Utilities|FlowControl|Switch|SwitchonENUM_CURVO_TipoGrate (Variables|Struttura|GetCURVO_TipoGrata)
            (:NewEnumerator0
              (Transformation|SetRelativeLocation _curvo_rollup "0.000000, 0,110.000000" false false))
            (:NewEnumerator1
              (Transformation|SetRelativeLocation _curvo_rollup "0, 0, 0" false false))))
        (:then_2
          (Components|StaticMesh|SetStaticMesh (Variables|Default|GetCURVE_AttaccoTubes) "/Game/Maps/Moduli/Mesh/Curvo/G_Curve_Tube.G_Curve_Tube"))))
    (:NewEnumerator3
      ;[1 1 1] Modulo a Quattro
      (CallFunction|HideTraps false)
      (Components|StaticMesh|SetStaticMesh (Variables|Default|GetQUATTRO_Roof) "/Game/Maps/Moduli/Mesh/Quattro/G_Four_Roof.G_Four_Roof")
      (Components|StaticMesh|SetStaticMesh (Variables|Default|GetQUATTRO_Floor) "/Game/Maps/Moduli/Mesh/Quattro/G_Four_Floor.G_Four_Floor")
      (Components|StaticMesh|SetStaticMesh (Variables|Default|GetQUATTRO_Columns) "/Game/Maps/Moduli/Mesh/Quattro/G_Four_Columns.G_Four_Columns")
      (Components|StaticMesh|SetStaticMesh (Variables|Default|GetQUATTRO_RoofHole) "/Game/Maps/Moduli/Mesh/Quattro/G_Four_RoofHole.G_Four_RoofHole")
      (Components|StaticMesh|SetStaticMesh (Variables|Default|GetQUATTRO_Tubes) "/Game/Maps/Moduli/Mesh/Quattro/G_Four_Tubes.G_Four_Tubes")
      (Components|StaticMesh|SetStaticMesh (Variables|Default|GetQUATTRO_FloorSkirting) "/Game/Maps/Moduli/Mesh/Quattro/G_Four_Floor_Skirting.G_Four_Floor_Skirting")
      (Rendering|SetVisibility (Variables|Default|GetQUATTRO_Plain) true false))))

(fn HideTraps
  (params (NewVisibility :type Boolean))
  (Rendering|SetVisibility (Variables|Default|GetAngleTrapFrontRight) NewVisibility false)
  (Rendering|SetVisibility (Variables|Default|GetAngleTrapBackLeft) NewVisibility false)
  (Rendering|SetVisibility (Variables|Default|GetAngleTrapBackRight) NewVisibility false)
  (Rendering|SetVisibility (Variables|Default|GetAngleTrapFrontLeft) NewVisibility false)
  (Rendering|SetVisibility (Variables|Default|GetTrappolaDavantiSinistraSystems) NewVisibility false)
  (Rendering|SetVisibility (Variables|Default|GetTrappolaCentraleSinistraSystems) NewVisibility false)
  (Rendering|SetVisibility (Variables|Default|GetTrappolaDavantiDestraSystems) NewVisibility false)
  (Rendering|SetVisibility (Variables|Default|GetTrappolaCentraleDestraSystems) NewVisibility false)
  (Rendering|SetVisibility (Variables|Default|GetTrappolaDietroDestraSystems) NewVisibility false)
  (Rendering|SetVisibility (Variables|Default|GetTrappolaDietroSinistraSystems) NewVisibility false))

(fn SetTraps
  (Utilities|FlowControl|Sequence))

(fn SetWallBases
  (bind _dritto_basewalltubesright (Variables|Default|GetDRITTO_BaseWallTubesRight))
  (bind _dritto_wallbaseleft (Variables|Default|GetDRITTO_WallBaseLeft))
  (bind _dritto_wallbaseright (Variables|Default|GetDRITTO_WallBaseRight))
  (bind _dritto_basewalltubesleft (Variables|Default|GetDRITTO_BaseWallTubesLeft))
  (switch Utilities|FlowControl|Switch|SwitchonENUM_DRITTO_WallBase (Variables|Struttura|GetDRITTO_TipoWallBaseLeft)
    (:NewEnumerator0
      (Components|StaticMesh|SetStaticMesh _dritto_wallbaseleft "/Game/Maps/Moduli/Mesh/Dritto/G_Straight_BaseWall_V1_002.G_Straight_BaseWall_V1_002")
      (Components|StaticMesh|SetStaticMesh _dritto_basewalltubesleft "/Game/Maps/Moduli/Mesh/Dritto/G_Straight_Side_Tube_V1_002.G_Straight_Side_Tube_V1_002"))
    (:NewEnumerator1
      (Components|StaticMesh|SetStaticMesh _dritto_wallbaseleft "/Game/Maps/Moduli/Mesh/Dritto/G_Straight_BaseWall_V2_002.G_Straight_BaseWall_V2_002")
      (Components|StaticMesh|SetStaticMesh _dritto_basewalltubesleft "/Game/Maps/Moduli/Mesh/Dritto/G_Straight_Side_Tube_V2_002.G_Straight_Side_Tube_V2_002"))
    (:NewEnumerator2
      (Components|StaticMesh|SetStaticMesh _dritto_wallbaseleft "/Game/Maps/Moduli/Mesh/Dritto/G_Straight_BaseWall_V3_4_002.G_Straight_BaseWall_V3_4_002")
      (Components|StaticMesh|SetStaticMesh _dritto_basewalltubesleft "/Game/Maps/Moduli/Mesh/Dritto/G_Straight_Side_Tube_V3_002.G_Straight_Side_Tube_V3_002"))
    (:NewEnumerator3
      (Components|StaticMesh|SetStaticMesh _dritto_wallbaseleft "/Game/Maps/Moduli/Mesh/Dritto/G_Straight_BaseWall_V3_4_002.G_Straight_BaseWall_V3_4_002")
      (Components|StaticMesh|SetStaticMesh _dritto_basewalltubesleft "/Game/Maps/Moduli/Mesh/Dritto/G_Straight_Side_Tube_V4_002.G_Straight_Side_Tube_V4_002"))
    (:NewEnumerator4
      (Components|StaticMesh|SetStaticMesh _dritto_wallbaseleft "/Game/Maps/Moduli/Mesh/Dritto/G_Straight_BaseWall_V3_4_002.G_Straight_BaseWall_V3_4_002")))
  (switch Utilities|FlowControl|Switch|SwitchonENUM_DRITTO_WallBase (Variables|Struttura|GetDRITTO_TipoWallBaseRight)
    (:NewEnumerator0
      (Components|StaticMesh|SetStaticMesh _dritto_wallbaseright "/Game/Maps/Moduli/Mesh/Dritto/G_Straight_BaseWall_V1_002.G_Straight_BaseWall_V1_002")
      (Components|StaticMesh|SetStaticMesh _dritto_basewalltubesright "/Game/Maps/Moduli/Mesh/Dritto/G_Straight_Side_Tube_V1_002.G_Straight_Side_Tube_V1_002"))
    (:NewEnumerator1
      (Components|StaticMesh|SetStaticMesh _dritto_wallbaseright "/Game/Maps/Moduli/Mesh/Dritto/G_Straight_BaseWall_V2_002.G_Straight_BaseWall_V2_002")
      (Components|StaticMesh|SetStaticMesh _dritto_basewalltubesright "/Game/Maps/Moduli/Mesh/Dritto/G_Straight_Side_Tube_V2_002.G_Straight_Side_Tube_V2_002"))
    (:NewEnumerator2
      (Components|StaticMesh|SetStaticMesh _dritto_wallbaseright "/Game/Maps/Moduli/Mesh/Dritto/G_Straight_BaseWall_V3_4_002.G_Straight_BaseWall_V3_4_002")
      (Components|StaticMesh|SetStaticMesh _dritto_basewalltubesright "/Game/Maps/Moduli/Mesh/Dritto/G_Straight_Side_Tube_V3_002.G_Straight_Side_Tube_V3_002"))
    (:NewEnumerator3
      (Components|StaticMesh|SetStaticMesh _dritto_wallbaseright "/Game/Maps/Moduli/Mesh/Dritto/G_Straight_BaseWall_V3_4_002.G_Straight_BaseWall_V3_4_002")
      (Components|StaticMesh|SetStaticMesh _dritto_basewalltubesright "/Game/Maps/Moduli/Mesh/Dritto/G_Straight_Side_Tube_V4_002.G_Straight_Side_Tube_V4_002"))
    (:NewEnumerator4
      (Components|StaticMesh|SetStaticMesh _dritto_wallbaseright "/Game/Maps/Moduli/Mesh/Dritto/G_Straight_BaseWall_V3_4_002.G_Straight_BaseWall_V3_4_002"))))

(fn SetLowerSideTubesPannels
  (bind _dritto_sidepannelsbassofrontright (Variables|Default|GetDRITTO_SidePannelsBassoFrontRight))
  (bind _dritto_sidepannelsbassobackleft (Variables|Default|GetDRITTO_SidePannelsBassoBackLeft))
  (bind _dritto_sidetubes_lowerbackleft (Variables|Default|GetDRITTO_SideTubes_LowerBackLeft))
  (bind _dritto_sidetubes_upperbackleft (Variables|Default|GetDRITTO_SideTubes_UpperBackLeft))
  (bind _dritto_sidetubes_lowerbackright (Variables|Default|GetDRITTO_SideTubes_LowerBackRight))
  (bind _dritto_sidetubes_upperbackright (Variables|Default|GetDRITTO_SideTubes_UpperBackRight))
  (bind _dritto_sidetubes_lowerfrontleft (Variables|Default|GetDRITTO_SideTubes_LowerFrontLeft))
  (bind _dritto_sidetubes_upperfrontleft (Variables|Default|GetDRITTO_SideTubes_UpperFrontLeft))
  (bind _dritto_sidetubes_lowerfrontright (Variables|Default|GetDRITTO_SideTubes_LowerFrontRight))
  (bind _dritto_sidetubes_upperfrontright (Variables|Default|GetDRITTO_SideTubes_UpperFrontRight))
  (bind _dritto_sidepannelsbassobackright (Variables|Default|GetDRITTO_SidePannelsBassoBackRight))
  (bind _dritto_sidepannelsbassofrontleft (Variables|Default|GetDRITTO_SidePannelsBassoFrontLeft))
  (Utilities|FlowControl|Sequence
    (:then_0
      (switch Utilities|FlowControl|Switch|SwitchonENUM_DRITTO_LowerSideTubes (Variables|PannelliBassi|GetDRITTO_TipoTubiBackLeft)
        (:NewEnumerator0
          (Components|StaticMesh|SetStaticMesh _dritto_sidetubes_lowerbackleft "/Game/Maps/Moduli/Mesh/Dritto/G_Straight_Side_Tube_Basso_Lower_V1_002.G_Straight_Side_Tube_Basso_Lower_V1_002")
          (Components|StaticMesh|SetStaticMesh _dritto_sidetubes_upperbackleft "/Game/Maps/Moduli/Mesh/Dritto/G_Straight_Side_Tube_Basso_Upper_V1_002.G_Straight_Side_Tube_Basso_Upper_V1_002"))
        (:NewEnumerator1
          (Components|StaticMesh|SetStaticMesh _dritto_sidetubes_lowerbackleft "/Game/Maps/Moduli/Mesh/Dritto/G_Straight_Side_Tube_Basso_Lower_V2_002.G_Straight_Side_Tube_Basso_Lower_V2_002")
          (Components|StaticMesh|SetStaticMesh _dritto_sidetubes_upperbackleft "/Game/Maps/Moduli/Mesh/Dritto/G_Straight_Side_Tube_Basso_Upper_V2_002.G_Straight_Side_Tube_Basso_Upper_V2_002")))
      (switch Utilities|FlowControl|Switch|SwitchonENUM_DRITTO_LowerSideTubes (Variables|PannelliBassi|GetDRITTO_TipoTubiBackRight)
        (:NewEnumerator0
          (Components|StaticMesh|SetStaticMesh _dritto_sidetubes_lowerbackright "/Game/Maps/Moduli/Mesh/Dritto/G_Straight_Side_Tube_Basso_Lower_V1_002.G_Straight_Side_Tube_Basso_Lower_V1_002")
          (Components|StaticMesh|SetStaticMesh _dritto_sidetubes_upperbackright "/Game/Maps/Moduli/Mesh/Dritto/G_Straight_Side_Tube_Basso_Upper_V1_002.G_Straight_Side_Tube_Basso_Upper_V1_002"))
        (:NewEnumerator1
          (Components|StaticMesh|SetStaticMesh _dritto_sidetubes_lowerbackright "/Game/Maps/Moduli/Mesh/Dritto/G_Straight_Side_Tube_Basso_Lower_V2_002.G_Straight_Side_Tube_Basso_Lower_V2_002")
          (Components|StaticMesh|SetStaticMesh _dritto_sidetubes_upperbackright "/Game/Maps/Moduli/Mesh/Dritto/G_Straight_Side_Tube_Basso_Upper_V2_002.G_Straight_Side_Tube_Basso_Upper_V2_002")))
      (switch Utilities|FlowControl|Switch|SwitchonENUM_DRITTO_LowerSideTubes (Variables|PannelliBassi|GetDRITTO_TipoTubiFrontLeft)
        (:NewEnumerator0
          (Components|StaticMesh|SetStaticMesh _dritto_sidetubes_lowerfrontleft "/Game/Maps/Moduli/Mesh/Dritto/G_Straight_Side_Tube_Basso_Lower_V1_002.G_Straight_Side_Tube_Basso_Lower_V1_002")
          (Components|StaticMesh|SetStaticMesh _dritto_sidetubes_upperfrontleft "/Game/Maps/Moduli/Mesh/Dritto/G_Straight_Side_Tube_Basso_Upper_V1_002.G_Straight_Side_Tube_Basso_Upper_V1_002"))
        (:NewEnumerator1
          (Components|StaticMesh|SetStaticMesh _dritto_sidetubes_lowerfrontleft "/Game/Maps/Moduli/Mesh/Dritto/G_Straight_Side_Tube_Basso_Lower_V2_002.G_Straight_Side_Tube_Basso_Lower_V2_002")
          (Components|StaticMesh|SetStaticMesh _dritto_sidetubes_upperfrontleft "/Game/Maps/Moduli/Mesh/Dritto/G_Straight_Side_Tube_Basso_Upper_V2_002.G_Straight_Side_Tube_Basso_Upper_V2_002")))
      (switch Utilities|FlowControl|Switch|SwitchonENUM_DRITTO_LowerSideTubes (Variables|PannelliBassi|GetDRITTO_TipoTubiFrontRight)
        (:NewEnumerator0
          (Components|StaticMesh|SetStaticMesh _dritto_sidetubes_lowerfrontright "/Game/Maps/Moduli/Mesh/Dritto/G_Straight_Side_Tube_Basso_Lower_V1_002.G_Straight_Side_Tube_Basso_Lower_V1_002")
          (Components|StaticMesh|SetStaticMesh _dritto_sidetubes_upperfrontright "/Game/Maps/Moduli/Mesh/Dritto/G_Straight_Side_Tube_Basso_Upper_V1_002.G_Straight_Side_Tube_Basso_Upper_V1_002"))
        (:NewEnumerator1
          (Components|StaticMesh|SetStaticMesh _dritto_sidetubes_lowerfrontright "/Game/Maps/Moduli/Mesh/Dritto/G_Straight_Side_Tube_Basso_Lower_V2_002.G_Straight_Side_Tube_Basso_Lower_V2_002")
          (Components|StaticMesh|SetStaticMesh _dritto_sidetubes_upperfrontright "/Game/Maps/Moduli/Mesh/Dritto/G_Straight_Side_Tube_Basso_Upper_V2_002.G_Straight_Side_Tube_Basso_Upper_V2_002"))))
    (:then_1
      (switch Utilities|FlowControl|Switch|SwitchonENUM_DRITTO_LowerSidePannel (Variables|PannelliBassi|GetDRITTO_TipoPannelliLowerBackLeft)
        (:NewEnumerator0
          (Components|StaticMesh|SetStaticMesh _dritto_sidepannelsbassobackleft "/Game/Maps/Moduli/Mesh/Dritto/G_Straight_Side_Pannel_V1_002.G_Straight_Side_Pannel_V1_002"))
        (:NewEnumerator1
          (Components|StaticMesh|SetStaticMesh _dritto_sidepannelsbassobackleft "/Game/Maps/Moduli/Mesh/Dritto/G_Straight_Side_Pannel_V2_002.G_Straight_Side_Pannel_V2_002"))
        (:NewEnumerator2
          (Components|StaticMesh|SetStaticMesh _dritto_sidepannelsbassobackleft "/Game/Maps/Moduli/Mesh/Dritto/G_Straight_Side_Pannel_V3_002.G_Straight_Side_Pannel_V3_002"))
        (:NewEnumerator3
          (Components|StaticMesh|SetStaticMesh _dritto_sidepannelsbassobackleft "/Game/Maps/Moduli/Mesh/Dritto/G_Straight_Side_Pannel_V4_002.G_Straight_Side_Pannel_V4_002")))
      (switch Utilities|FlowControl|Switch|SwitchonENUM_DRITTO_LowerSidePannel (Variables|PannelliBassi|GetDRITTO_TipoPannelliLowerBackRight)
        (:NewEnumerator0
          (Components|StaticMesh|SetStaticMesh _dritto_sidepannelsbassobackright "/Game/Maps/Moduli/Mesh/Dritto/G_Straight_Side_Pannel_V1_002.G_Straight_Side_Pannel_V1_002"))
        (:NewEnumerator1
          (Components|StaticMesh|SetStaticMesh _dritto_sidepannelsbassobackright "/Game/Maps/Moduli/Mesh/Dritto/G_Straight_Side_Pannel_V2_002.G_Straight_Side_Pannel_V2_002"))
        (:NewEnumerator2
          (Components|StaticMesh|SetStaticMesh _dritto_sidepannelsbassobackright "/Game/Maps/Moduli/Mesh/Dritto/G_Straight_Side_Pannel_V3_002.G_Straight_Side_Pannel_V3_002"))
        (:NewEnumerator3
          (Components|StaticMesh|SetStaticMesh _dritto_sidepannelsbassobackright "/Game/Maps/Moduli/Mesh/Dritto/G_Straight_Side_Pannel_V4_002.G_Straight_Side_Pannel_V4_002")))
      (switch Utilities|FlowControl|Switch|SwitchonENUM_DRITTO_LowerSidePannel (Variables|PannelliBassi|GetDRITTO_TipoPannelliLowerFrontLeft)
        (:NewEnumerator0
          (Components|StaticMesh|SetStaticMesh _dritto_sidepannelsbassofrontleft "/Game/Maps/Moduli/Mesh/Dritto/G_Straight_Side_Pannel_V1_002.G_Straight_Side_Pannel_V1_002"))
        (:NewEnumerator1
          (Components|StaticMesh|SetStaticMesh _dritto_sidepannelsbassofrontleft "/Game/Maps/Moduli/Mesh/Dritto/G_Straight_Side_Pannel_V2_002.G_Straight_Side_Pannel_V2_002"))
        (:NewEnumerator2
          (Components|StaticMesh|SetStaticMesh _dritto_sidepannelsbassofrontleft "/Game/Maps/Moduli/Mesh/Dritto/G_Straight_Side_Pannel_V3_002.G_Straight_Side_Pannel_V3_002"))
        (:NewEnumerator3
          (Components|StaticMesh|SetStaticMesh _dritto_sidepannelsbassofrontleft "/Game/Maps/Moduli/Mesh/Dritto/G_Straight_Side_Pannel_V4_002.G_Straight_Side_Pannel_V4_002")))
      (switch Utilities|FlowControl|Switch|SwitchonENUM_DRITTO_LowerSidePannel (Variables|PannelliBassi|GetDRITTO_TipoPannelliLowerFrontRight)
        (:NewEnumerator0
          (Components|StaticMesh|SetStaticMesh _dritto_sidepannelsbassofrontright "/Game/Maps/Moduli/Mesh/Dritto/G_Straight_Side_Pannel_V1_002.G_Straight_Side_Pannel_V1_002"))
        (:NewEnumerator1
          (Components|StaticMesh|SetStaticMesh _dritto_sidepannelsbassofrontright "/Game/Maps/Moduli/Mesh/Dritto/G_Straight_Side_Pannel_V2_002.G_Straight_Side_Pannel_V2_002"))
        (:NewEnumerator2
          (Components|StaticMesh|SetStaticMesh _dritto_sidepannelsbassofrontright "/Game/Maps/Moduli/Mesh/Dritto/G_Straight_Side_Pannel_V3_002.G_Straight_Side_Pannel_V3_002"))
        (:NewEnumerator3
          (Components|StaticMesh|SetStaticMesh _dritto_sidepannelsbassofrontright "/Game/Maps/Moduli/Mesh/Dritto/G_Straight_Side_Pannel_V4_002.G_Straight_Side_Pannel_V4_002"))))))

(fn SetSkirtings
  (bind _dritto_skirtingrooffront (Variables|Default|GetDRITTO_SkirtingRoofFront))
  (bind _dritto_columnbackleft (Variables|Default|GetDRITTO_ColumnBackLeft))
  (bind _dritto_columnbackright (Variables|Default|GetDRITTO_ColumnBackRight))
  (bind _dritto_skirtingfloorfront (Variables|Default|GetDRITTO_SkirtingFloorFront))
  (bind _dritto_skirtingroofback (Variables|Default|GetDRITTO_SkirtingRoofBack))
  (bind _dritto_skirtingfloorback (Variables|Default|GetDRITTO_SkirtingFloorBack))
  (bind _dritto_columnfrontleft (Variables|Default|GetDRITTO_ColumnFrontLeft))
  (bind _dritto_columnfrontright (Variables|Default|GetDRITTO_ColumnFrontRight))
  (Utilities|FlowControl|Sequence
    (:then_0
      (switch Utilities|FlowControl|Switch|SwitchonENUM_DRITTO_Columns (Variables|Struttura|GetDRITTO_TipoAttaccoFront)
        (:NewEnumerator2
          (Components|StaticMesh|SetStaticMesh _dritto_columnfrontleft "/Game/Maps/Moduli/Mesh/Dritto/G_Straight_Column_Static_002.G_Straight_Column_Static_002")
          (Components|StaticMesh|SetStaticMesh _dritto_columnfrontright "/Game/Maps/Moduli/Mesh/Dritto/G_Straight_Column_Static_002.G_Straight_Column_Static_002")
          (Components|StaticMesh|SetStaticMesh _dritto_skirtingrooffront "/Game/Maps/Moduli/Mesh/Dritto/G_Straight_Attacco_Roof_Skirting_002.G_Straight_Attacco_Roof_Skirting_002")
          (Components|StaticMesh|SetStaticMesh _dritto_skirtingfloorfront "/Game/Maps/Moduli/Mesh/Dritto/G_Straight_Attacco_Floor_Skirting_002.G_Straight_Attacco_Floor_Skirting_002"))
        (:NewEnumerator3
          (Components|StaticMesh|SetStaticMesh _dritto_columnfrontleft "/Game/Maps/Moduli/Mesh/Dritto/G_Straight_Column_Personalizable_002.G_Straight_Column_Personalizable_002")
          (Components|StaticMesh|SetStaticMesh _dritto_columnfrontright "/Game/Maps/Moduli/Mesh/Dritto/G_Straight_Column_Personalizable_002.G_Straight_Column_Personalizable_002")
          (Components|StaticMesh|SetStaticMesh _dritto_skirtingrooffront "/Game/Maps/Moduli/Mesh/Dritto/G_Straight_Attacco_Roof_Skirting_002.G_Straight_Attacco_Roof_Skirting_002")
          (Components|StaticMesh|SetStaticMesh _dritto_skirtingfloorfront "/Game/Maps/Moduli/Mesh/Dritto/G_Straight_Attacco_Floor_Skirting_002.G_Straight_Attacco_Floor_Skirting_002")
          (Components|StaticMesh|SetStaticMesh (Variables|Default|GetDRITTO_SkirtingTubeFrontLeft) "/Game/Maps/Moduli/Mesh/Dritto/G_Straight_Attacco_Tube_001.G_Straight_Attacco_Tube_001")
          (Components|StaticMesh|SetStaticMesh (Variables|Default|GetDRITTO_SkirtingTubeFrontRight) "/Game/Maps/Moduli/Mesh/Dritto/G_Straight_Attacco_Tube_001.G_Straight_Attacco_Tube_001"))
        (:NewEnumerator4
          (Components|StaticMesh|SetStaticMesh (Variables|Default|GetDRITTO_SkirtingRoofFront) "/Game/Maps/Moduli/Mesh/Dritto/G_Straight_Attacco_Roof_Skirting_002.G_Straight_Attacco_Roof_Skirting_002")
          (Components|StaticMesh|SetStaticMesh (Variables|Default|GetDRITTO_SkirtingFloorFront) "/Game/Maps/Moduli/Mesh/Dritto/G_Straight_Attacco_Floor_Skirting_002.G_Straight_Attacco_Floor_Skirting_002"))))
    (:then_1
      (switch Utilities|FlowControl|Switch|SwitchonENUM_DRITTO_Columns (Variables|Struttura|GetDRITTO_TipoAttaccoBack)
        (:NewEnumerator2
          (Components|StaticMesh|SetStaticMesh _dritto_columnbackleft "/Game/Maps/Moduli/Mesh/Dritto/G_Straight_Column_Static_002.G_Straight_Column_Static_002")
          (Components|StaticMesh|SetStaticMesh _dritto_columnbackright "/Game/Maps/Moduli/Mesh/Dritto/G_Straight_Column_Static_002.G_Straight_Column_Static_002")
          (Components|StaticMesh|SetStaticMesh _dritto_skirtingroofback "/Game/Maps/Moduli/Mesh/Dritto/G_Straight_Attacco_Roof_Skirting_002.G_Straight_Attacco_Roof_Skirting_002")
          (Components|StaticMesh|SetStaticMesh _dritto_skirtingfloorback "/Game/Maps/Moduli/Mesh/Dritto/G_Straight_Attacco_Floor_Skirting_002.G_Straight_Attacco_Floor_Skirting_002"))
        (:NewEnumerator3
          (Components|StaticMesh|SetStaticMesh _dritto_columnbackleft "/Game/Maps/Moduli/Mesh/Dritto/G_Straight_Column_Personalizable_002.G_Straight_Column_Personalizable_002")
          (Components|StaticMesh|SetStaticMesh _dritto_columnbackright "/Game/Maps/Moduli/Mesh/Dritto/G_Straight_Column_Personalizable_002.G_Straight_Column_Personalizable_002")
          (Components|StaticMesh|SetStaticMesh _dritto_skirtingroofback "/Game/Maps/Moduli/Mesh/Dritto/G_Straight_Attacco_Roof_Skirting_002.G_Straight_Attacco_Roof_Skirting_002")
          (Components|StaticMesh|SetStaticMesh _dritto_skirtingfloorback "/Game/Maps/Moduli/Mesh/Dritto/G_Straight_Attacco_Floor_Skirting_002.G_Straight_Attacco_Floor_Skirting_002")
          (Components|StaticMesh|SetStaticMesh (Variables|Default|GetDRITTO_SkirtingTubeBackLeft) "/Game/Maps/Moduli/Mesh/Dritto/G_Straight_Attacco_Tube_001.G_Straight_Attacco_Tube_001")
          (Components|StaticMesh|SetStaticMesh (Variables|Default|GetDRITTO_SkirtingTubeBackRight) "/Game/Maps/Moduli/Mesh/Dritto/G_Straight_Attacco_Tube_001.G_Straight_Attacco_Tube_001"))
        (:NewEnumerator4
          (Components|StaticMesh|SetStaticMesh (Variables|Default|GetDRITTO_SkirtingRoofBack) "/Game/Maps/Moduli/Mesh/Dritto/G_Straight_Attacco_Roof_Skirting_002.G_Straight_Attacco_Roof_Skirting_002")
          (Components|StaticMesh|SetStaticMesh (Variables|Default|GetDRITTO_SkirtingFloorBack) "/Game/Maps/Moduli/Mesh/Dritto/G_Straight_Attacco_Floor_Skirting_002.G_Straight_Attacco_Floor_Skirting_002"))))))

(fn SetColumnSlots
  (bind _dritto_columntubesbackleft (Variables|Default|GetDRITTO_ColumnTubesBackLeft))
  (bind _dritto_columntubesfrontright (Variables|Default|GetDRITTO_ColumnTubesFrontRight))
  (bind _dritto_columnpannelbackleft (Variables|Default|GetDRITTO_ColumnPannelBackLeft))
  (bind _dritto_columnpannelbackright (Variables|Default|GetDRITTO_ColumnPannelBackRight))
  (bind _dritto_columnpannelfrontleft (Variables|Default|GetDRITTO_ColumnPannelFrontLeft))
  (bind _dritto_columnpannelfrontright (Variables|Default|GetDRITTO_ColumnPannelFrontRight))
  (bind _dritto_columntubesbackright (Variables|Default|GetDRITTO_ColumnTubesBackRight))
  (bind _dritto_columntubesfrontleft (Variables|Default|GetDRITTO_ColumnTubesFrontLeft))
  (Utilities|FlowControl|Sequence
    (:then_0
      (if (Utilities|Enum|Equal(Enum) (Variables|Struttura|GetDRITTO_TipoAttaccoBack) "NewEnumerator3")
        ;[1 1 1] Pannels
        (switch Utilities|FlowControl|Switch|SwitchonENUM_DRITTO_ColumnPannel (Variables|Columns|GetDRITTO_TipoColumnPannelBackLeft)
          (:NewEnumerator0
            (Components|StaticMesh|SetStaticMesh _dritto_columnpannelbackleft "/Game/Maps/Moduli/Mesh/Dritto/G_Straight_ColumnPannel_V1_002.G_Straight_ColumnPannel_V1_002" :!label _label))
          (:NewEnumerator1
            (Components|StaticMesh|SetStaticMesh _dritto_columnpannelbackleft "/Game/Maps/Moduli/Mesh/Dritto/G_Straight_ColumnPannel_V2_002.G_Straight_ColumnPannel_V2_002"))
          (:NewEnumerator2
            (if (Utilities|Enum|Equal(Enum) (Variables|Columns|GetDRITTO_TipoColumnTubesBackLeft) "NewEnumerator2")
              (goto _label)
              (else
                (Components|StaticMesh|SetStaticMesh _dritto_columnpannelbackleft "/Game/Maps/Moduli/Mesh/Dritto/G_Straight_ColumnPannel_V3_002.G_Straight_ColumnPannel_V3_002")))))
        (switch Utilities|FlowControl|Switch|SwitchonENUM_DRITTO_ColumnPannel (Variables|Columns|GetDRITTO_TipoColumnPannelBackRight)
          (:NewEnumerator0
            (Components|StaticMesh|SetStaticMesh _dritto_columnpannelbackright "/Game/Maps/Moduli/Mesh/Dritto/G_Straight_ColumnPannel_V1_002.G_Straight_ColumnPannel_V1_002" :!label _label_2))
          (:NewEnumerator1
            (Components|StaticMesh|SetStaticMesh _dritto_columnpannelbackright "/Game/Maps/Moduli/Mesh/Dritto/G_Straight_ColumnPannel_V2_002.G_Straight_ColumnPannel_V2_002"))
          (:NewEnumerator2
            (if (Utilities|Enum|Equal(Enum) (Variables|Columns|GetDRITTO_TipoColumnTubesBackRight) "NewEnumerator2")
              (goto _label_2)
              (else
                (Components|StaticMesh|SetStaticMesh _dritto_columnpannelbackright "/Game/Maps/Moduli/Mesh/Dritto/G_Straight_ColumnPannel_V3_002.G_Straight_ColumnPannel_V3_002")))))
        (switch Utilities|FlowControl|Switch|SwitchonENUM_DRITTO_ColumnTubes (Variables|Columns|GetDRITTO_TipoColumnTubesBackLeft)
          (:NewEnumerator0
            (Components|StaticMesh|SetStaticMesh _dritto_columntubesbackleft "/Game/Maps/Moduli/Mesh/Dritto/G_Straight_ColumnTube_V1_002.G_Straight_ColumnTube_V1_002" :!label _label_3))
          (:NewEnumerator1
            (Components|StaticMesh|SetStaticMesh _dritto_columntubesbackleft "/Game/Maps/Moduli/Mesh/Dritto/G_Straight_ColumnTube_V2_002.G_Straight_ColumnTube_V2_002"))
          (:NewEnumerator2
            (if (Utilities|Enum|Equal(Enum) (Variables|Columns|GetDRITTO_TipoColumnPannelBackLeft) "NewEnumerator2")
              (goto _label_3)
              (else
                (Components|StaticMesh|SetStaticMesh _dritto_columntubesbackleft "/Game/Maps/Moduli/Mesh/Dritto/G_Straight_ColumnTube_V3_002.G_Straight_ColumnTube_V3_002")))))
        (switch Utilities|FlowControl|Switch|SwitchonENUM_DRITTO_ColumnTubes (Variables|Columns|GetDRITTO_TipoColumnTubesBackRight)
          (:NewEnumerator0
            (Components|StaticMesh|SetStaticMesh _dritto_columntubesbackright "/Game/Maps/Moduli/Mesh/Dritto/G_Straight_ColumnTube_V1_002.G_Straight_ColumnTube_V1_002" :!label _label_4))
          (:NewEnumerator1
            (Components|StaticMesh|SetStaticMesh _dritto_columntubesbackright "/Game/Maps/Moduli/Mesh/Dritto/G_Straight_ColumnTube_V2_002.G_Straight_ColumnTube_V2_002"))
          (:NewEnumerator2
            (if (Utilities|Enum|Equal(Enum) (Variables|Columns|GetDRITTO_TipoColumnPannelBackRight) "NewEnumerator2")
              (goto _label_4)
              (else
                (Components|StaticMesh|SetStaticMesh _dritto_columntubesbackright "/Game/Maps/Moduli/Mesh/Dritto/G_Straight_ColumnTube_V3_002.G_Straight_ColumnTube_V3_002")))))))
    (:then_1
      (if (Utilities|Enum|Equal(Enum) (Variables|Struttura|GetDRITTO_TipoAttaccoFront) "NewEnumerator3")
        ;[1 1 1] Pannels
        (switch Utilities|FlowControl|Switch|SwitchonENUM_DRITTO_ColumnPannel (Variables|Columns|GetDRITTO_TipoColumnPannelFrontLeft)
          (:NewEnumerator0
            (Components|StaticMesh|SetStaticMesh _dritto_columnpannelfrontleft "/Game/Maps/Moduli/Mesh/Dritto/G_Straight_ColumnPannel_V1_002.G_Straight_ColumnPannel_V1_002")
            (switch Utilities|FlowControl|Switch|SwitchonENUM_DRITTO_ColumnPannel (Variables|Columns|GetDRITTO_TipoColumnPannelFrontRight) :!label _label_5
              (:NewEnumerator0
                (Components|StaticMesh|SetStaticMesh _dritto_columnpannelfrontright "/Game/Maps/Moduli/Mesh/Dritto/G_Straight_ColumnPannel_V1_002.G_Straight_ColumnPannel_V1_002" :!label _label_6))
              (:NewEnumerator1
                (Components|StaticMesh|SetStaticMesh _dritto_columnpannelfrontright "/Game/Maps/Moduli/Mesh/Dritto/G_Straight_ColumnPannel_V2_002.G_Straight_ColumnPannel_V2_002"))
              (:NewEnumerator2
                (if (Utilities|Enum|Equal(Enum) (Variables|Columns|GetDRITTO_TipoColumnTubesFrontRight) "NewEnumerator2")
                  (goto _label_6)
                  (else
                    (Components|StaticMesh|SetStaticMesh _dritto_columnpannelfrontright "/Game/Maps/Moduli/Mesh/Dritto/G_Straight_ColumnPannel_V3_002.G_Straight_ColumnPannel_V3_002")))))
            (switch Utilities|FlowControl|Switch|SwitchonENUM_DRITTO_ColumnTubes (Variables|Columns|GetDRITTO_TipoColumnTubesFrontLeft)
              (:NewEnumerator0
                (Components|StaticMesh|SetStaticMesh _dritto_columntubesfrontleft "/Game/Maps/Moduli/Mesh/Dritto/G_Straight_ColumnTube_V1_002.G_Straight_ColumnTube_V1_002" :!label _label_7))
              (:NewEnumerator1
                (Components|StaticMesh|SetStaticMesh _dritto_columntubesfrontleft "/Game/Maps/Moduli/Mesh/Dritto/G_Straight_ColumnTube_V2_002.G_Straight_ColumnTube_V2_002"))
              (:NewEnumerator2
                (if (Utilities|Enum|Equal(Enum) (Variables|Columns|GetDRITTO_TipoColumnPannelFrontLeft) "NewEnumerator2")
                  (goto _label_7)
                  (else
                    (Components|StaticMesh|SetStaticMesh _dritto_columntubesfrontleft "/Game/Maps/Moduli/Mesh/Dritto/G_Straight_ColumnTube_V3_002.G_Straight_ColumnTube_V3_002")))))
            (switch Utilities|FlowControl|Switch|SwitchonENUM_DRITTO_ColumnTubes (Variables|Columns|GetDRITTO_TipoColumnTubesFrontRight)
              (:NewEnumerator0
                (Components|StaticMesh|SetStaticMesh _dritto_columntubesfrontright "/Game/Maps/Moduli/Mesh/Dritto/G_Straight_ColumnTube_V1_002.G_Straight_ColumnTube_V1_002" :!label _label_8))
              (:NewEnumerator1
                (Components|StaticMesh|SetStaticMesh _dritto_columntubesfrontright "/Game/Maps/Moduli/Mesh/Dritto/G_Straight_ColumnTube_V2_002.G_Straight_ColumnTube_V2_002"))
              (:NewEnumerator2
                (if (Utilities|Enum|Equal(Enum) (Variables|Columns|GetDRITTO_TipoColumnPannelFrontRight) "NewEnumerator2")
                  (goto _label_8)
                  (else
                    (Components|StaticMesh|SetStaticMesh _dritto_columntubesfrontright "/Game/Maps/Moduli/Mesh/Dritto/G_Straight_ColumnTube_V3_002.G_Straight_ColumnTube_V3_002"))))))
          (:NewEnumerator1
            (Components|StaticMesh|SetStaticMesh _dritto_columnpannelfrontleft "/Game/Maps/Moduli/Mesh/Dritto/G_Straight_ColumnPannel_V2_002.G_Straight_ColumnPannel_V2_002")
            (goto _label_5))
          (:NewEnumerator2
            (if (not (Utilities|Enum|Equal(Enum) (Variables|Columns|GetDRITTO_TipoColumnTubesFrontLeft) "NewEnumerator2"))
              (Components|StaticMesh|SetStaticMesh _dritto_columnpannelfrontleft "/Game/Maps/Moduli/Mesh/Dritto/G_Straight_ColumnPannel_V3_002.G_Straight_ColumnPannel_V3_002")
              (goto _label_5))))))))