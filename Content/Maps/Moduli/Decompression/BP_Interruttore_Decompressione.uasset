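; Decompression airlock switch that, on interaction, alternates an entrance and exit door while swapping the level streaming on either side.
; Closes the open door, waits briefly, toggles the two streaming volumes, then loops on the newly enabled volume's loading-assets check before opening the opposite door.
; An interact widget, created hidden at BeginPlay, flashes briefly when the switch is in sight.
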(event EventInteract
  (bind _streamingvolumeingresso (Variables|Default|GetStreamingVolumeIngresso))
  (bind _streamingvolumeuscita (Variables|Default|GetStreamingVolumeUscita))
  ;[1 1 1] Apertura, carico scarico e chiusura
  (if (Variables|/Game/Maps/Moduli/Porta/BP_Porta_Oggetto.BP_Porta_Oggetto_C|GetOpen (Variables|Default|GetPortaIngresso))
    ;[1 1 1] Ingresso aperta, Uscita chiusa
    (Default|CloseDoor (Variables|Default|GetPortaIngresso))
    (Utilities|FlowControl|Delay 2.0)
    (Variables|/Script/Engine.LevelStreamingVolume|SetbDisabled (Variables|Default|GetStreamingVolumeIngresso) true)
    (Variables|/Script/Engine.LevelStreamingVolume|SetbDisabled _streamingvolumeuscita false)
    (while (stale _returnvalue)
      (bind _returnvalue (Class|AssetRegistry|IsLoadingAssets(Message) _streamingvolumeuscita)))
    (Default|OpenDoor (Variables|Default|GetPortaUscita))
    (else
      ;[1 1 1] Uscita aperta, Ingresso chiuso
      (Default|CloseDoor (Variables|Default|GetPortaUscita))
      (Utilities|FlowControl|Delay 2.0)
      (Variables|/Script/Engine.LevelStreamingVolume|SetbDisabled (Variables|Default|GetStreamingVolumeUscita) true)
      (Variables|/Script/Engine.LevelStreamingVolume|SetbDisabled _streamingvolumeingresso false)
      (while (stale _returnvalue_2)
        (bind _returnvalue_2 (Class|AssetRegistry|IsLoadingAssets(Message) _streamingvolumeingresso)))
      (Default|OpenDoor (Variables|Default|GetPortaIngresso)))))

(event EventInSight
  (params (IsInSight? :type Boolean))
  (bind _playerwidget (Variables|Default|GetPlayerWidget))
  ;[1 1 1] InSight
  (if IsInSight?
    (Widget|SetVisibility _playerwidget "Visible")
    (Utilities|FlowControl|Delay 0.5)
    (Widget|SetVisibility _playerwidget "Hidden")
    (else
      (Widget|SetVisibility (Variables|Default|GetPlayerWidget) "Hidden"))))

(event EventBeginPlay
  ;[1 1 1] Create interact Widget
  (bind _returnvalue (UserInterface|CreateWidget "/Game/Maps/Moduli/Porta/WIDGET_Interact.WIDGET_Interact_C" (Game|GetPlayerController 0)))
  (bind _output_get (Variables|Default|SetPlayerWidget _returnvalue))
  (UserInterface|Viewport|AddtoViewport _returnvalue 0)
  (Widget|SetVisibility _output_get "Hidden"))

(fn ConstructionScript)