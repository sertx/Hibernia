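; BP_ModuloPorta is a modular double door whose two leaves slide along their local X axis.
; Open and Close events play and reverse the DoorsMovement timeline when CanOpen is set, with separate distance tracks driving the left and right doors.
; When UsesTriggerBox is set, overlaps beginning and ending on DoorTrigger call those events automatically, without filtering the overlapping actor.
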(event OnComponentBeginOverlap(DoorTrigger)
  (params (OverlappedComponent :type Primitive%20Component%20Object%20Reference) (OtherActor :type Actor%20Object%20Reference) (OtherComp :type Primitive%20Component%20Object%20Reference) (OtherBodyIndex :type Integer) (bFromSweep :type Boolean) (SweepResult :type Hit%20Result%20Structure%20%28by%20ref%29))
  (if (Variables|Default|GetUsesTriggerBox)
    (CallFunction|Open)))

(event OnComponentEndOverlap(DoorTrigger)
  (params (OverlappedComponent :type Primitive%20Component%20Object%20Reference) (OtherActor :type Actor%20Object%20Reference) (OtherComp :type Primitive%20Component%20Object%20Reference) (OtherBodyIndex :type Integer))
  (if (Variables|Default|GetUsesTriggerBox)
    (CallFunction|Close)))

(event Custom|Open
  (bind _leftdoor (Variables|Default|GetLeftDoor))
  (bind _rightdoor (Variables|Default|GetRightDoor))
  (bind _relativelocation (Variables|/Script/Engine.SceneComponent|GetRelativeLocation _leftdoor))
  (bind _relativelocation_2 (Variables|/Script/Engine.SceneComponent|GetRelativeLocation _rightdoor))
  (if (Variables|Default|GetCanOpen)
    (bind (_direction _distanceright _distanceleft) (Timeline|DoorsMovement Play)
      (:Update
        (Transformation|SetRelativeLocation _leftdoor (Math|Vector|MakeVector _distanceleft (.y _relativelocation) (.z _relativelocation)) false false)
        (Transformation|SetRelativeLocation _rightdoor (Math|Vector|MakeVector _distanceright (.y _relativelocation_2) (.z _relativelocation_2)) false false)))))

(event Custom|Close
  (bind _leftdoor (Variables|Default|GetLeftDoor))
  (bind _rightdoor (Variables|Default|GetRightDoor))
  (bind _relativelocation (Variables|/Script/Engine.SceneComponent|GetRelativeLocation _leftdoor))
  (bind _relativelocation_2 (Variables|/Script/Engine.SceneComponent|GetRelativeLocation _rightdoor))
  (if (Variables|Default|GetCanOpen)
    (bind (_direction _distanceright _distanceleft) (Timeline|DoorsMovement Reverse)
      (:Update
        (Transformation|SetRelativeLocation _leftdoor (Math|Vector|MakeVector _distanceleft (.y _relativelocation) (.z _relativelocation)) false false)
        (Transformation|SetRelativeLocation _rightdoor (Math|Vector|MakeVector _distanceright (.y _relativelocation_2) (.z _relativelocation_2)) false false)))))

(fn ConstructionScript)