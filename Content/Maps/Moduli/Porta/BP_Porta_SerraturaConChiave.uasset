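; BP_Porta_SerraturaConChiave is a door lock that opens its linked door when the player has the key.
; It creates a hidden interaction widget at BeginPlay, briefly showing it when InSight reports true and hiding it otherwise.
; On Interact, it checks Key1PickedUp on the ThirdPersonCharacter and, if set, casts PortaCollegata to BP_Porta_Oggetto and calls OpenDoor.
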(event EventInteract
  (bind _asthird_person_character (Utilities|Casting|CastToThirdPersonCharacter (Game|Player|GetPlayerPawn 0)))
  (if (Variables|/Game/Character/ThirdPersonCharacter.ThirdPersonCharacter_C|GetKey1PickedUp _asthird_person_character)
    (bind _asbp_porta_oggetto (Utilities|Casting|CastToBP_Porta_Oggetto (Variables|Default|GetPortaCollegata)))
    (Default|OpenDoor _asbp_porta_oggetto)))

(event EventInSight
  (params (IsInSight? :type Boolean))
  (bind _playerwidget (Variables|Default|GetPlayerWidget))
  (if IsInSight?
    (Widget|SetVisibility _playerwidget "Visible")
    (Utilities|FlowControl|Delay 0.5)
    (Widget|SetVisibility _playerwidget "Hidden")
    (else
      (Widget|SetVisibility (Variables|Default|GetPlayerWidget) "Hidden"))))

(event EventBeginPlay
  (bind _returnvalue (UserInterface|CreateWidget "/Game/Maps/Moduli/Porta/WIDGET_Interact.WIDGET_Interact_C" (Game|GetPlayerController 0)))
  (bind _output_get (Variables|Default|SetPlayerWidget _returnvalue))
  (UserInterface|Viewport|AddtoViewport _returnvalue 0)
  (Widget|SetVisibility _output_get "Hidden"))

(fn ConstructionScript)