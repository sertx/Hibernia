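; Modular straight corridor piece (Modulo Dritto) for level building, assembled entirely in the construction script from per-side type variables.
; Each option adds an instance to a shared instanced-mesh component at a placeholder component's world transform, covering roof, walls, bases, tubes, panels and skirtings.
; Trap walls fill each slot with a side trap or warmer.
; Personalizable attachments add column slots, where closed panels with on-floor tubes fall back to open panels and V1 tubes.
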(fn ConstructionScript
  (bind _grataangletrap (Variables|Default|GetGrataAngleTrap))
  (bind _dritto_roof (Variables|Default|GetDRITTO_Roof))
  (bind _dritto_wallleft (Variables|Default|GetDRITTO_WallLeft))
  (bind _dritto_wallright (Variables|Default|GetDRITTO_WallRight))
  (bind _dritto_uppersidegridleft (Variables|Default|GetDRITTO_UpperSideGridLeft))
  (bind _dritto_uppersidegridright (Variables|Default|GetDRITTO_UpperSideGridRight))
  (bind _returnvalue (Transformation|GetWorldTransform _dritto_roof))
  (bind _returnvalue_2 (Transformation|GetWorldTransform _dritto_wallleft))
  (bind _returnvalue_3 (Transformation|GetWorldTransform _dritto_uppersidegridright))
  (bind _returnvalue_4 (Transformation|GetWorldTransform _dritto_uppersidegridleft))
  (bind _returnvalue_5 (Transformation|GetWorldTransform _dritto_wallright))
  ;[1 1 1] Gestione Tipo Modulo Dritto
  (Utilities|FlowControl|Sequence
    (:then_0
      (switch Utilities|FlowControl|Switch|SwitchonENUM_DRITTO_Roof (Variables|Struttura|GetDRITTO_TipoRoof)
        (:NewEnumerator0
          (Class|InstancedStaticMeshComponent|AddInstanceWorldSpace (Variables|Default|GetRoofLibero) _returnvalue))
        (:NewEnumerator1
          (Class|InstancedStaticMeshComponent|AddInstanceWorldSpace (Variables|Default|GetRoofWithGrid) _returnvalue)
          (Class|InstancedStaticMeshComponent|AddInstanceWorldSpace (Variables|Default|GetRoofGrid) (Transformation|GetWorldTransform (Variables|Default|GetDRITTO_RoofGrid)))))
      (Components|StaticMesh|SetStaticMesh (Variables|Default|GetDRITTO_Floor) "/Game/Maps/Moduli/Mesh/Dritto/G_Straight_Floor_001.G_Straight_Floor_001"))
    (:then_1
      (switch Utilities|FlowControl|Switch|SwitchonENUM_DRITTO_Muri (Variables|Struttura|GetDRITTO_TipoMuroLeft)
        (:NewEnumerator4
          (Class|InstancedStaticMeshComponent|AddInstanceWorldSpace (Variables|Default|GetWallLibero) _returnvalue_2))
        (:NewEnumerator5
          (Class|InstancedStaticMeshComponent|AddInstanceWorldSpace (Variables|Default|GetWallTrappole) _returnvalue_2)))
      (switch Utilities|FlowControl|Switch|SwitchonENUM_DRITTO_Muri (Variables|Struttura|GetDRITTO_TipoMuroRight)
        (:NewEnumerator4
          (Class|InstancedStaticMeshComponent|AddInstanceWorldSpace (Variables|Default|GetWallLibero) _returnvalue_5))
        (:NewEnumerator5
          (Class|InstancedStaticMeshComponent|AddInstanceWorldSpace (Variables|Default|GetWallTrappole) _returnvalue_5))))
    (:then_2
      (CallFunction|SetTraps))
    (:then_3
      (CallFunction|SetWallBases))
    (:then_4
      (CallFunction|SetLowerSideTubesPannels))
    (:then_5
      (CallFunction|SetSkirtings))
    (:then_6
      (CallFunction|SetColumnSlots))
    (:then_7
      (Class|InstancedStaticMeshComponent|AddInstanceWorldSpace _grataangletrap (Transformation|GetWorldTransform (Variables|Default|GetDRITTO_GrataAngleTrapLeft)))
      (Class|InstancedStaticMeshComponent|AddInstanceWorldSpace _grataangletrap (Transformation|GetWorldTransform (Variables|Default|GetDRITTO_GrataAngleTrapRight))))
    (:then_8
      (switch Utilities|FlowControl|Switch|SwitchonENUM_DRITTO_SideGrid (Variables|Struttura|GetDRITTO_TipoSideGridLeft)
        (:NewEnumerator0
          (Class|InstancedStaticMeshComponent|AddInstanceWorldSpace (Variables|Default|GetSideGridGrid) _returnvalue_4))
        (:NewEnumerator1
          (Class|InstancedStaticMeshComponent|AddInstanceWorldSpace (Variables|Default|GetSideGridBroken) _returnvalue_4))
        (:NewEnumerator2
          (Class|InstancedStaticMeshComponent|AddInstanceWorldSpace (Variables|Default|GetSideGridTubes) _returnvalue_4)))
      (switch Utilities|FlowControl|Switch|SwitchonENUM_DRITTO_SideGrid (Variables|Struttura|GetDRITTO_TipoSideGridRight)
        (:NewEnumerator0
          (Class|InstancedStaticMeshComponent|AddInstanceWorldSpace (Variables|Default|GetSideGridGrid) _returnvalue_3))
        (:NewEnumerator1
          (Class|InstancedStaticMeshComponent|AddInstanceWorldSpace (Variables|Default|GetSideGridBroken) _returnvalue_3))
        (:NewEnumerator2
          (Class|InstancedStaticMeshComponent|AddInstanceWorldSpace (Variables|Default|GetSideGridTubes) _returnvalue_3))))))

(fn SetTraps
  (bind _dritto_trapfrontleft (Variables|Default|GetDRITTO_TrapFrontLeft))
  (bind _dritto_trapmidleft (Variables|Default|GetDRITTO_TrapMidLeft))
  (bind _dritto_trapbackleft (Variables|Default|GetDRITTO_TrapBackLeft))
  (bind _dritto_trapfrontright (Variables|Default|GetDRITTO_TrapFrontRight))
  (bind _dritto_trapmidright (Variables|Default|GetDRITTO_TrapMidRight))
  (bind _dritto_trapbackright (Variables|Default|GetDRITTO_TrapBackRight))
  (bind _returnvalue (Transformation|GetWorldTransform _dritto_trapbackright))
  (bind _returnvalue_2 (Transformation|GetWorldTransform _dritto_trapfrontleft))
  (bind _returnvalue_3 (Transformation|GetWorldTransform _dritto_trapmidleft))
  (bind _returnvalue_4 (Transformation|GetWorldTransform _dritto_trapbackleft))
  (bind _returnvalue_5 (Transformation|GetWorldTransform _dritto_trapfrontright))
  (bind _returnvalue_6 (Transformation|GetWorldTransform _dritto_trapmidright))
  (Utilities|FlowControl|Sequence
    (:then_0
      (switch Utilities|FlowControl|Switch|SwitchonENUM_DRITTO_Muri (Variables|Struttura|GetDRITTO_TipoMuroLeft)
        (:NewEnumerator5
          (if (Variables|Traps|GetDRITTO_TipoTrappolaFrontLeft)
            (Class|InstancedStaticMeshComponent|AddInstanceWorldSpace (Variables|Default|GetSideTrap) _returnvalue_2)
            (else
              (Class|InstancedStaticMeshComponent|AddInstanceWorldSpace (Variables|Default|GetWarmer) _returnvalue_2)))
          (if (Variables|Traps|GetDRITTO_TipoTrappoleMidLeft)
            (Class|InstancedStaticMeshComponent|AddInstanceWorldSpace (Variables|Default|GetSideTrap) _returnvalue_3)
            (else
              (Class|InstancedStaticMeshComponent|AddInstanceWorldSpace (Variables|Default|GetWarmer) _returnvalue_3)))
          (if (Variables|Traps|GetDRITTO_TipoTrappolaBackLeft)
            (Class|InstancedStaticMeshComponent|AddInstanceWorldSpace (Variables|Default|GetSideTrap) _returnvalue_4)
            (else
              (Class|InstancedStaticMeshComponent|AddInstanceWorldSpace (Variables|Default|GetWarmer) _returnvalue_4))))))
    (:then_1
      (switch Utilities|FlowControl|Switch|SwitchonENUM_DRITTO_Muri (Variables|Struttura|GetDRITTO_TipoMuroRight)
        (:NewEnumerator5
          (if (Variables|Traps|GetDRITTO_TipoTrappolaFrontRight)
            (Class|InstancedStaticMeshComponent|AddInstanceWorldSpace (Variables|Default|GetSideTrap) _returnvalue_5)
            (else
              (Class|InstancedStaticMeshComponent|AddInstanceWorldSpace (Variables|Default|GetWarmer) _returnvalue_5)))
          (if (Variables|Traps|GetDRITTO_TipoTrappolaMidRight)
            (Class|InstancedStaticMeshComponent|AddInstanceWorldSpace (Variables|Default|GetSideTrap) _returnvalue_6)
            (else
              (Class|InstancedStaticMeshComponent|AddInstanceWorldSpace (Variables|Default|GetWarmer) _returnvalue_6)))
          (if (Variables|Traps|GetDRITTO_TipoTrappolaBackRight)
            (Class|InstancedStaticMeshComponent|AddInstanceWorldSpace (Variables|Default|GetSideTrap) _returnvalue)
            (else
              (Class|InstancedStaticMeshComponent|AddInstanceWorldSpace (Variables|Default|GetWarmer) _returnvalue))))))))

(fn SetWallBases
  (bind _dritto_basewalltubesright (Variables|Default|GetDRITTO_BaseWallTubesRight))
  (bind _dritto_wallbaseleft (Variables|Default|GetDRITTO_WallBaseLeft))
  (bind _dritto_wallbaseright (Variables|Default|GetDRITTO_WallBaseRight))
  (bind _dritto_basewalltubesleft (Variables|Default|GetDRITTO_BaseWallTubesLeft))
  (bind _returnvalue (Transformation|GetWorldTransform _dritto_wallbaseleft))
  (bind _returnvalue_2 (Transformation|GetWorldTransform _dritto_wallbaseright))
  (bind _returnvalue_3 (Transformation|GetWorldTransform _dritto_basewalltubesright))
  (bind _returnvalue_4 (Transformation|GetWorldTransform _dritto_basewalltubesleft))
  (switch Utilities|FlowControl|Switch|SwitchonENUM_DRITTO_WallBase (Variables|Struttura|GetDRITTO_TipoWallBaseLeft)
    (:NewEnumerator0
      (Class|InstancedStaticMeshComponent|AddInstanceWorldSpace (Variables|Default|GetWallBaseV1) _returnvalue)
      (Class|InstancedStaticMeshComponent|AddInstanceWorldSpace (Variables|Default|GetSideTubesV1) _returnvalue_4))
    (:NewEnumerator1
      (Class|InstancedStaticMeshComponent|AddInstanceWorldSpace (Variables|Default|GetWallBaseV2) _returnvalue)
      (Class|InstancedStaticMeshComponent|AddInstanceWorldSpace (Variables|Default|GetSideTubesV2) _returnvalue_4))
    (:NewEnumerator2
      (Class|InstancedStaticMeshComponent|AddInstanceWorldSpace (Variables|Default|GetWallBaseV3) _returnvalue)
      (Class|InstancedStaticMeshComponent|AddInstanceWorldSpace (Variables|Default|GetSideTubesV3) _returnvalue_4))
    (:NewEnumerator3
      (Class|InstancedStaticMeshComponent|AddInstanceWorldSpace (Variables|Default|GetWallBaseV3) _returnvalue)
      (Class|InstancedStaticMeshComponent|AddInstanceWorldSpace (Variables|Default|GetSideTubesV4) _returnvalue_4))
    (:NewEnumerator4
      (Class|InstancedStaticMeshComponent|AddInstanceWorldSpace (Variables|Default|GetWallBaseV3) _returnvalue)))
  (switch Utilities|FlowControl|Switch|SwitchonENUM_DRITTO_WallBase (Variables|Struttura|GetDRITTO_TipoWallBaseRight)
    (:NewEnumerator0
      (Class|InstancedStaticMeshComponent|AddInstanceWorldSpace (Variables|Default|GetWallBaseV1) _returnvalue_2)
      (Class|InstancedStaticMeshComponent|AddInstanceWorldSpace (Variables|Default|GetSideTubesV1) _returnvalue_3))
    (:NewEnumerator1
      (Class|InstancedStaticMeshComponent|AddInstanceWorldSpace (Variables|Default|GetWallBaseV2) _returnvalue_2)
      (Class|InstancedStaticMeshComponent|AddInstanceWorldSpace (Variables|Default|GetSideTubesV2) _returnvalue_3))
    (:NewEnumerator2
      (Class|InstancedStaticMeshComponent|AddInstanceWorldSpace (Variables|Default|GetWallBaseV3) _returnvalue_2)
      (Class|InstancedStaticMeshComponent|AddInstanceWorldSpace (Variables|Default|GetSideTubesV3) _returnvalue_3))
    (:NewEnumerator3
      (Class|InstancedStaticMeshComponent|AddInstanceWorldSpace (Variables|Default|GetWallBaseV3) _returnvalue_2)
      (Class|InstancedStaticMeshComponent|AddInstanceWorldSpace (Variables|Default|GetSideTubesV4) _returnvalue_3))
    (:NewEnumerator4
      (Class|InstancedStaticMeshComponent|AddInstanceWorldSpace (Variables|Default|GetWallBaseV3) _returnvalue_2))))

(fn SetLowerSideTubesPannels
  (bind _dritto_sidepannelsbassofrontright (Variables|Default|GetDRITTO_SidePannelsBassoFrontRight))
  (bind _dritto_sidepannelsbassobackleft (Variables|Default|GetDRITTO_SidePannelsBassoBackLeft))
  (bind _dritto_sidepannelsbassobackright (Variables|Default|GetDRITTO_SidePannelsBassoBackRight))
  (bind _dritto_sidepannelsbassofrontleft (Variables|Default|GetDRITTO_SidePannelsBassoFrontLeft))
  (bind _returnvalue (Transformation|GetWorldTransform _dritto_sidepannelsbassofrontright))
  (bind _returnvalue_2 (Transformation|GetWorldTransform _dritto_sidepannelsbassobackleft))
  (bind _returnvalue_3 (Transformation|GetWorldTransform _dritto_sidepannelsbassobackright))
  (bind _returnvalue_4 (Transformation|GetWorldTransform _dritto_sidepannelsbassofrontleft))
  (Utilities|FlowControl|Sequence
    (:then_0
      ;[1 1 1] Tubes
      (Class|InstancedStaticMeshComponent|AddInstanceWorldSpace (Variables|Default|GetLowerSideTubesDown) (Transformation|GetWorldTransform (Variables|Default|GetDRITTO_SideTubes_LowerBackLeft)))
      (Class|InstancedStaticMeshComponent|AddInstanceWorldSpace (Variables|Default|GetLowerSideTubesUp) (Transformation|GetWorldTransform (Variables|Default|GetDRITTO_SideTubes_UpperBackLeft)))
      (Class|InstancedStaticMeshComponent|AddInstanceWorldSpace (Variables|Default|GetLowerSideTubesDown) (Transformation|GetWorldTransform (Variables|Default|GetDRITTO_SideTubes_LowerBackRight)))
      (Class|InstancedStaticMeshComponent|AddInstanceWorldSpace (Variables|Default|GetLowerSideTubesUp) (Transformation|GetWorldTransform (Variables|Default|GetDRITTO_SideTubes_UpperBackRight)))
      (Class|InstancedStaticMeshComponent|AddInstanceWorldSpace (Variables|Default|GetLowerSideTubesDown) (Transformation|GetWorldTransform (Variables|Default|GetDRITTO_SideTubes_LowerFrontLeft)))
      (Class|InstancedStaticMeshComponent|AddInstanceWorldSpace (Variables|Default|GetLowerSideTubesUp) (Transformation|GetWorldTransform (Variables|Default|GetDRITTO_SideTubes_UpperFrontLeft)))
      (Class|InstancedStaticMeshComponent|AddInstanceWorldSpace (Variables|Default|GetLowerSideTubesDown) (Transformation|GetWorldTransform (Variables|Default|GetDRITTO_SideTubes_LowerFrontRight)))
      (Class|InstancedStaticMeshComponent|AddInstanceWorldSpace (Variables|Default|GetLowerSideTubesUp) (Transformation|GetWorldTransform (Variables|Default|GetDRITTO_SideTubes_UpperFrontRight))))
    (:then_1
      ;[1 1 1] Pannels
      (switch Utilities|FlowControl|Switch|SwitchonENUM_DRITTO_LowerSidePannel (Variables|PannelliBassi|GetDRITTO_TipoPannelliLowerBackLeft)
        (:NewEnumerator0
          (Class|InstancedStaticMeshComponent|AddInstanceWorldSpace (Variables|Default|GetSidePannelV1) _returnvalue_2))
        (:NewEnumerator1
          (Class|InstancedStaticMeshComponent|AddInstanceWorldSpace (Variables|Default|GetSidePannelV2) _returnvalue_2))
        (:NewEnumerator2
          (Class|InstancedStaticMeshComponent|AddInstanceWorldSpace (Variables|Default|GetSidePannelV3) _returnvalue_2))
        (:NewEnumerator3
          (Class|InstancedStaticMeshComponent|AddInstanceWorldSpace (Variables|Default|GetSidePannelV4) _returnvalue_2)))
      (switch Utilities|FlowControl|Switch|SwitchonENUM_DRITTO_LowerSidePannel (Variables|PannelliBassi|GetDRITTO_TipoPannelliLowerBackRight)
        (:NewEnumerator0
          (Class|InstancedStaticMeshComponent|AddInstanceWorldSpace (Variables|Default|GetSidePannelV1) _returnvalue_3))
        (:NewEnumerator1
          (Class|InstancedStaticMeshComponent|AddInstanceWorldSpace (Variables|Default|GetSidePannelV2) _returnvalue_3))
        (:NewEnumerator2
          (Class|InstancedStaticMeshComponent|AddInstanceWorldSpace (Variables|Default|GetSidePannelV3) _returnvalue_3))
        (:NewEnumerator3
          (Class|InstancedStaticMeshComponent|AddInstanceWorldSpace (Variables|Default|GetSidePannelV4) _returnvalue_3)))
      (switch Utilities|FlowControl|Switch|SwitchonENUM_DRITTO_LowerSidePannel (Variables|PannelliBassi|GetDRITTO_TipoPannelliLowerFrontLeft)
        (:NewEnumerator0
          (Class|InstancedStaticMeshComponent|AddInstanceWorldSpace (Variables|Default|GetSidePannelV1) _returnvalue_4))
        (:NewEnumerator1
          (Class|InstancedStaticMeshComponent|AddInstanceWorldSpace (Variables|Default|GetSidePannelV2) _returnvalue_4))
        (:NewEnumerator2
          (Class|InstancedStaticMeshComponent|AddInstanceWorldSpace (Variables|Default|GetSidePannelV3) _returnvalue_4))
        (:NewEnumerator3
          (Class|InstancedStaticMeshComponent|AddInstanceWorldSpace (Variables|Default|GetSidePannelV4) _returnvalue_4)))
      (switch Utilities|FlowControl|Switch|SwitchonENUM_DRITTO_LowerSidePannel (Variables|PannelliBassi|GetDRITTO_TipoPannelliLowerFrontRight)
        (:NewEnumerator0
          (Class|InstancedStaticMeshComponent|AddInstanceWorldSpace (Variables|Default|GetSidePannelV1) _returnvalue))
        (:NewEnumerator1
          (Class|InstancedStaticMeshComponent|AddInstanceWorldSpace (Variables|Default|GetSidePannelV2) _returnvalue))
        (:NewEnumerator2
          (Class|InstancedStaticMeshComponent|AddInstanceWorldSpace (Variables|Default|GetSidePannelV3) _returnvalue))
        (:NewEnumerator3
          (Class|InstancedStaticMeshComponent|AddInstanceWorldSpace (Variables|Default|GetSidePannelV4) _returnvalue))))))

(fn SetSkirtings
  (bind _dritto_skirtingrooffront (Variables|Default|GetDRITTO_SkirtingRoofFront))
  (bind _dritto_columnbackleft (Variables|Default|GetDRITTO_ColumnBackLeft))
  (bind _dritto_columnbackright (Variables|Default|GetDRITTO_ColumnBackRight))
  (bind _dritto_skirtingfloorfront (Variables|Default|GetDRITTO_SkirtingFloorFront))
  (bind _dritto_skirtingroofback (Variables|Default|GetDRITTO_SkirtingRoofBack))
  (bind _dritto_skirtingfloorback (Variables|Default|GetDRITTO_SkirtingFloorBack))
  (bind _dritto_columnfrontleft (Variables|Default|GetDRITTO_ColumnFrontLeft))
  (bind _dritto_columnfrontright (Variables|Default|GetDRITTO_ColumnFrontRight))
  (bind _returnvalue (Transformation|GetWorldTransform _dritto_skirtingfloorback))
  (bind _returnvalue_2 (Transformation|GetWorldTransform _dritto_columnbackleft))
  (bind _returnvalue_3 (Transformation|GetWorldTransform _dritto_columnbackright))
  (bind _returnvalue_4 (Transformation|GetWorldTransform _dritto_skirtingroofback))
  (bind _returnvalue_5 (Transformation|GetWorldTransform _dritto_columnfrontleft))
  (bind _returnvalue_6 (Transformation|GetWorldTransform _dritto_columnfrontright))
  (bind _returnvalue_7 (Transformation|GetWorldTransform _dritto_skirtingrooffront))
  (bind _returnvalue_8 (Transformation|GetWorldTransform _dritto_skirtingfloorfront))
  (Utilities|FlowControl|Sequence
    (:then_0
      (switch Utilities|FlowControl|Switch|SwitchonENUM_DRITTO_Columns (Variables|Struttura|GetDRITTO_TipoAttaccoFront)
        (:NewEnumerator2
          (Class|InstancedStaticMeshComponent|AddInstanceWorldSpace (Variables|Default|GetColumnStatic) _returnvalue_5)
          (Class|InstancedStaticMeshComponent|AddInstanceWorldSpace (Variables|Default|GetColumnStatic) _returnvalue_6)
          (Class|InstancedStaticMeshComponent|AddInstanceWorldSpace (Variables|Default|GetColumnStatic) _returnvalue_7)
          (Class|InstancedStaticMeshComponent|AddInstanceWorldSpace (Variables|Default|GetColumnStatic) _returnvalue_8))
        (:NewEnumerator3
          (Class|InstancedStaticMeshComponent|AddInstanceWorldSpace (Variables|Default|GetColumnPersonalizable) _returnvalue_5)
          (Class|InstancedStaticMeshComponent|AddInstanceWorldSpace (Variables|Default|GetColumnPersonalizable) _returnvalue_6)
          (Class|InstancedStaticMeshComponent|AddInstanceWorldSpace (Variables|Default|GetColumnPersonalizable) _returnvalue_7)
          (Class|InstancedStaticMeshComponent|AddInstanceWorldSpace (Variables|Default|GetColumnPersonalizable) _returnvalue_8)
          (Class|InstancedStaticMeshComponent|AddInstanceWorldSpace (Variables|Default|GetTubeSkirting) (Transformation|GetWorldTransform (Variables|Default|GetDRITTO_SkirtingTubeFrontLeft)))
          (Class|InstancedStaticMeshComponent|AddInstanceWorldSpace (Variables|Default|GetTubeSkirting) (Transformation|GetWorldTransform (Variables|Default|GetDRITTO_SkirtingTubeFrontRight))))
        (:NewEnumerator4
          (Class|InstancedStaticMeshComponent|AddInstanceWorldSpace (Variables|Default|GetRoofSkirting) (Transformation|GetWorldTransform (Variables|Default|GetDRITTO_SkirtingRoofFront)))
          (Class|InstancedStaticMeshComponent|AddInstanceWorldSpace (Variables|Default|GetFloorSkirting) (Transformation|GetWorldTransform (Variables|Default|GetDRITTO_SkirtingFloorFront))))))
    (:then_1
      (switch Utilities|FlowControl|Switch|SwitchonENUM_DRITTO_Columns (Variables|Struttura|GetDRITTO_TipoAttaccoBack)
        (:NewEnumerator2
          (Class|InstancedStaticMeshComponent|AddInstanceWorldSpace (Variables|Default|GetColumnStatic) _returnvalue_2)
          (Class|InstancedStaticMeshComponent|AddInstanceWorldSpace (Variables|Default|GetColumnStatic) _returnvalue_3)
          (Class|InstancedStaticMeshComponent|AddInstanceWorldSpace (Variables|Default|GetColumnStatic) _returnvalue_4)
          (Class|InstancedStaticMeshComponent|AddInstanceWorldSpace (Variables|Default|GetColumnStatic) _returnvalue))
        (:NewEnumerator3
          (Class|InstancedStaticMeshComponent|AddInstanceWorldSpace (Variables|Default|GetColumnPersonalizable) _returnvalue_2)
          (Class|InstancedStaticMeshComponent|AddInstanceWorldSpace (Variables|Default|GetColumnPersonalizable) _returnvalue_3)
          (Class|InstancedStaticMeshComponent|AddInstanceWorldSpace (Variables|Default|GetColumnPersonalizable) _returnvalue_4)
          (Class|InstancedStaticMeshComponent|AddInstanceWorldSpace (Variables|Default|GetColumnPersonalizable) _returnvalue)
          (Class|InstancedStaticMeshComponent|AddInstanceWorldSpace (Variables|Default|GetTubeSkirting) (Transformation|GetWorldTransform (Variables|Default|GetDRITTO_SkirtingTubeBackLeft)))
          (Class|InstancedStaticMeshComponent|AddInstanceWorldSpace (Variables|Default|GetTubeSkirting) (Transformation|GetWorldTransform (Variables|Default|GetDRITTO_SkirtingTubeBackRight))))
        (:NewEnumerator4
          (Class|InstancedStaticMeshComponent|AddInstanceWorldSpace (Variables|Default|GetRoofSkirting) (Transformation|GetWorldTransform (Variables|Default|GetDRITTO_SkirtingRoofBack)))
          (Class|InstancedStaticMeshComponent|AddInstanceWorldSpace (Variables|Default|GetFloorSkirting) (Transformation|GetWorldTransform (Variables|Default|GetDRITTO_SkirtingFloorBack))))))))

(fn SetColumnSlots
  (bind _dritto_columntubesbackleft (Variables|Default|GetDRITTO_ColumnTubesBackLeft))
  (bind _dritto_columntubesfrontright (Variables|Default|GetDRITTO_ColumnTubesFrontRight))
  (bind _dritto_columnpannelbackleft (Variables|Default|GetDRITTO_ColumnPannelBackLeft))
  (bind _dritto_columnpannelbackright (Variables|Default|GetDRITTO_ColumnPannelBackRight))
  (bind _dritto_columnpannelfrontleft (Variables|Default|GetDRITTO_ColumnPannelFrontLeft))
  (bind _dritto_columnpannelfrontright (Variables|Default|GetDRITTO_ColumnPannelFrontRight))
  (bind _dritto_columntubesbackright (Variables|Default|GetDRITTO_ColumnTubesBackRight))
  (bind _dritto_columntubesfrontleft (Variables|Default|GetDRITTO_ColumnTubesFrontLeft))
  (bind _returnvalue (Transformation|GetWorldTransform _dritto_columnpannelfrontright))
  (bind _returnvalue_2 (Transformation|GetWorldTransform _dritto_columnpannelbackleft))
  (bind _returnvalue_3 (Transformation|GetWorldTransform _dritto_columnpannelbackright))
  (bind _returnvalue_4 (Transformation|GetWorldTransform _dritto_columnpannelfrontleft))
  (bind _returnvalue_5 (Transformation|GetWorldTransform _dritto_columntubesfrontright))
  (bind _returnvalue_6 (Transformation|GetWorldTransform _dritto_columntubesbackleft))
  (bind _returnvalue_7 (Transformation|GetWorldTransform _dritto_columntubesbackright))
  (bind _returnvalue_8 (Transformation|GetWorldTransform _dritto_columntubesfrontleft))
  (Utilities|FlowControl|Sequence
    (:then_0
      (if (Utilities|Enum|Equal(Enum) (Variables|Struttura|GetDRITTO_TipoAttaccoBack) "NewEnumerator3")
        ;[1 1 1] Pannels
        (switch Utilities|FlowControl|Switch|SwitchonENUM_DRITTO_ColumnPannel (Variables|Columns|GetDRITTO_TipoColumnPannelBackLeft)
          (:NewEnumerator0
            (Class|InstancedStaticMeshComponent|AddInstanceWorldSpace (Variables|Default|GetColumnPannelOpen) _returnvalue_2 :!label _label))
          (:NewEnumerator1
            (Class|InstancedStaticMeshComponent|AddInstanceWorldSpace (Variables|Default|GetColumnPannelMidway) _returnvalue_2))
          (:NewEnumerator2
            (if (Utilities|Enum|Equal(Enum) (Variables|Columns|GetDRITTO_TipoColumnTubesBackLeft) "NewEnumerator2")
              (goto _label)
              (else
                (Class|InstancedStaticMeshComponent|AddInstanceWorldSpace (Variables|Default|GetColumnPannelClosed) _returnvalue_2)))))
        (switch Utilities|FlowControl|Switch|SwitchonENUM_DRITTO_ColumnPannel (Variables|Columns|GetDRITTO_TipoColumnPannelBackRight)
          (:NewEnumerator0
            (Class|InstancedStaticMeshComponent|AddInstanceWorldSpace (Variables|Default|GetColumnPannelOpen) _returnvalue_3 :!label _label_2))
          (:NewEnumerator1
            (Class|InstancedStaticMeshComponent|AddInstanceWorldSpace (Variables|Default|GetColumnPannelMidway) _returnvalue_3))
          (:NewEnumerator2
            (if (Utilities|Enum|Equal(Enum) (Variables|Columns|GetDRITTO_TipoColumnTubesBackRight) "NewEnumerator2")
              (goto _label_2)
              (else
                (Class|InstancedStaticMeshComponent|AddInstanceWorldSpace (Variables|Default|GetColumnPannelClosed) _returnvalue_3)))))
        (switch Utilities|FlowControl|Switch|SwitchonENUM_DRITTO_ColumnTubes (Variables|Columns|GetDRITTO_TipoColumnTubesBackLeft)
          (:NewEnumerator0
            (Class|InstancedStaticMeshComponent|AddInstanceWorldSpace (Variables|Default|GetColumnTubesV1) _returnvalue_6 :!label _label_3))
          (:NewEnumerator1
            (Class|InstancedStaticMeshComponent|AddInstanceWorldSpace (Variables|Default|GetColumnTubesV2) _returnvalue_6))
          (:NewEnumerator2
            (if (Utilities|Enum|Equal(Enum) (Variables|Columns|GetDRITTO_TipoColumnPannelBackLeft) "NewEnumerator2")
              (goto _label_3)
              (else
                (Class|InstancedStaticMeshComponent|AddInstanceWorldSpace (Variables|Default|GetColumnTubesOnFloor) _returnvalue_6)))))
        (switch Utilities|FlowControl|Switch|SwitchonENUM_DRITTO_ColumnTubes (Variables|Columns|GetDRITTO_TipoColumnTubesBackRight)
          (:NewEnumerator0
            (Class|InstancedStaticMeshComponent|AddInstanceWorldSpace (Variables|Default|GetColumnTubesV1) _returnvalue_7 :!label _label_4))
          (:NewEnumerator1
            (Class|InstancedStaticMeshComponent|AddInstanceWorldSpace (Variables|Default|GetColumnTubesV2) _returnvalue_7))
          (:NewEnumerator2
            (if (Utilities|Enum|Equal(Enum) (Variables|Columns|GetDRITTO_TipoColumnPannelBackRight) "NewEnumerator2")
              (goto _label_4)
              (else
                (Class|InstancedStaticMeshComponent|AddInstanceWorldSpace (Variables|Default|GetColumnTubesOnFloor) _returnvalue_7)))))))
    (:then_1
      (if (Utilities|Enum|Equal(Enum) (Variables|Struttura|GetDRITTO_TipoAttaccoFront) "NewEnumerator3")
        ;[1 1 1] Pannels
        (switch Utilities|FlowControl|Switch|SwitchonENUM_DRITTO_ColumnPannel (Variables|Columns|GetDRITTO_TipoColumnPannelFrontLeft)
          (:NewEnumerator0
            (Class|InstancedStaticMeshComponent|AddInstanceWorldSpace (Variables|Default|GetColumnPannelOpen) _returnvalue_4 :!label _label_5))
          (:NewEnumerator1
            (Class|InstancedStaticMeshComponent|AddInstanceWorldSpace (Variables|Default|GetColumnPannelMidway) _returnvalue_4))
          (:NewEnumerator2
            (if (Utilities|Enum|Equal(Enum) (Variables|Columns|GetDRITTO_TipoColumnTubesFrontLeft) "NewEnumerator2")
              (goto _label_5)
              (else
                (Class|InstancedStaticMeshComponent|AddInstanceWorldSpace (Variables|Default|GetColumnPannelClosed) _returnvalue_4)))))
        (switch Utilities|FlowControl|Switch|SwitchonENUM_DRITTO_ColumnPannel (Variables|Columns|GetDRITTO_TipoColumnPannelFrontRight)
          (:NewEnumerator0
            (Class|InstancedStaticMeshComponent|AddInstanceWorldSpace (Variables|Default|GetColumnPannelOpen) _returnvalue :!label _label_6))
          (:NewEnumerator1
            (Class|InstancedStaticMeshComponent|AddInstanceWorldSpace (Variables|Default|GetColumnPannelMidway) _returnvalue))
          (:NewEnumerator2
            (if (Utilities|Enum|Equal(Enum) (Variables|Columns|GetDRITTO_TipoColumnTubesFrontRight) "NewEnumerator2")
              (goto _label_6)
              (else
                (Class|InstancedStaticMeshComponent|AddInstanceWorldSpace (Variables|Default|GetColumnPannelClosed) _returnvalue)))))
        (switch Utilities|FlowControl|Switch|SwitchonENUM_DRITTO_ColumnTubes (Variables|Columns|GetDRITTO_TipoColumnTubesFrontLeft)
          (:NewEnumerator0
            (Class|InstancedStaticMeshComponent|AddInstanceWorldSpace (Variables|Default|GetColumnTubesV1) _returnvalue_8 :!label _label_7))
          (:NewEnumerator1
            (Class|InstancedStaticMeshComponent|AddInstanceWorldSpace (Variables|Default|GetColumnTubesV2) _returnvalue_8))
          (:NewEnumerator2
            (if (Utilities|Enum|Equal(Enum) (Variables|Columns|GetDRITTO_TipoColumnPannelFrontLeft) "NewEnumerator2")
              (goto _label_7)
              (else
                (Class|InstancedStaticMeshComponent|AddInstanceWorldSpace (Variables|Default|GetColumnTubesOnFloor) _returnvalue_8)))))
        (switch Utilities|FlowControl|Switch|SwitchonENUM_DRITTO_ColumnTubes (Variables|Columns|GetDRITTO_TipoColumnTubesFrontRight)
          (:NewEnumerator0
            (Class|InstancedStaticMeshComponent|AddInstanceWorldSpace (Variables|Default|GetColumnTubesV1) _returnvalue_5 :!label _label_8))
          (:NewEnumerator1
            (Class|InstancedStaticMeshComponent|AddInstanceWorldSpace (Variables|Default|GetColumnTubesV2) _returnvalue_5))
          (:NewEnumerator2
            (if (Utilities|Enum|Equal(Enum) (Variables|Columns|GetDRITTO_TipoColumnPannelFrontRight) "NewEnumerator2")
              (goto _label_8)
              (else
                (Class|InstancedStaticMeshComponent|AddInstanceWorldSpace (Variables|Default|GetColumnTubesOnFloor) _returnvalue_5)))))))))