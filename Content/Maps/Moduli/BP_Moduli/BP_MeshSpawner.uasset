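; BP_MeshSpawner is a module Blueprint holding instanced mesh components for two straight wall variants, free (Libero) and trap (Trappole).
; ClearAllInstances empties both components.
; SpawnMesh takes a mesh type and transform but is unwired, and the construction script is empty.
; The disconnected switch would clear the matching component before adding one world-space instance, leaving only the latest.
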(event Custom|SpawnMesh
  (params (Mesh :type MeshesEnum%20Enum :default "NewEnumerator0") (Transform :type Transform)))

(fn ConstructionScript)

(fn ClearAllInstances
  (for _array_element (Utilities|Array|MakeArray (Variables|Default|GetDRITTO_WallTrappole) (Variables|Default|GetDRITTO_WallLibero))
    (Components|InstancedStaticMesh|ClearInstances _array_element)))