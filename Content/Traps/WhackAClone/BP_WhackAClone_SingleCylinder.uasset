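; A single trap cylinder for Whack-A-Clone that slams down when the player stands in its collision box while the trap is active.
; Overlap events track the player, and Tick starts the MoveDown timeline whenever it is idle.
; The timeline drives the cylinder's absolute world Z, overriding the vertical offset applied at BeginPlay.
; At the bottom it spawns an explosion at a reference actor, pauses briefly, then retracts at half speed.
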(event OnComponentBeginOverlap(CollisionBox)
  (params (OverlappedComponent :type Primitive%20Component%20Object%20Reference) (OtherActor :type Actor%20Object%20Reference) (OtherComp :type Primitive%20Component%20Object%20Reference) (OtherBodyIndex :type Integer) (bFromSweep :type Boolean) (SweepResult :type Hit%20Result%20Structure%20%28by%20ref%29))
  (if (== OtherActor (Variables|Default|GetPlayer))
    (Variables|Default|SetOverlapping true)))

(event OnComponentEndOverlap(CollisionBox)
  (params (OverlappedComponent :type Primitive%20Component%20Object%20Reference) (OtherActor :type Actor%20Object%20Reference) (OtherComp :type Primitive%20Component%20Object%20Reference) (OtherBodyIndex :type Integer))
  (if (== OtherActor (Variables|Default|GetPlayer))
    (Variables|Default|SetOverlapping false)))

(event EventTick
  (params (DeltaSeconds :type Float%20%28single-precision%29))
  (bind _movedown (Variables|Default|GetMoveDown))
  (bind _cylinder (Variables|Default|GetCylinder))
  (bind _returnvalue (Transformation|GetWorldLocation _cylinder))
  (if (and (Variables|Default|GetActive) (Variables|Default|GetOverlapping))
    (if (not (Audio|Components|Audio|IsPlaying _movedown))
      (bind (_direction _cylindermovedown) (Timeline|MoveDown PlayFromStart)
        (:Update
          (Transformation|SetWorldLocation _cylinder (Math|Vector|MakeVector (.x _returnvalue) (.y _returnvalue) _cylindermovedown) false false))
        (:Finished
          (if (Utilities|Enum|Equal(Enum) _direction "Forward")
            (Effects|SpawnEmitteratLocation "/Game/StarterContent/Particles/P_Explosion.P_Explosion" (Transformation|GetActorLocation (Variables|Default|GetParticleSpawnPoint)))
            (Utilities|FlowControl|Delay 0.3)
            (Components|Timeline|SetPlayRate _movedown 0.5)
            (Timeline|MoveDown ReverseFromEnd)
            (else
              (Components|Timeline|SetPlayRate _movedown 1.0))))))))

(event EventBeginPlay
  (bind _asthird_person_character (Utilities|Casting|CastToThirdPersonCharacter (Game|Player|GetPlayerPawn 0)))
  (Variables|Default|SetPlayer _asthird_person_character)
  (Transformation|AddWorldOffset (Variables|Default|GetCylinder) (Math|Vector|MakeVector 0.0 0.0 (Variables|Default|GetCylinderVerticalOffset)) false false))

(fn ConstructionScript)