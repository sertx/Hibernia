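; Nitrogen (Azoto) trap that intermittently fires left and right emitters and kills the player character on contact.
; While Enabled, Tick drives chained Delays that repeatedly activate both emitters after a fixed wait and deactivate them after Frequency.
; CollisionDetector calls Muori (die) on an entering ThirdPersonCharacter only if both emitters are active.
; The check runs only on begin overlap, so activation does not affect characters already inside.
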(event OnComponentBeginOverlap(CollisionDetector)
  (params (OverlappedComponent :type Primitive%20Component%20Object%20Reference) (OtherActor :type Actor%20Object%20Reference) (OtherComp :type Primitive%20Component%20Object%20Reference) (OtherBodyIndex :type Integer) (bFromSweep :type Boolean) (SweepResult :type Hit%20Result%20Structure%20%28by%20ref%29))
  (if (and (Components|Activation|IsActive (Variables|Default|GetLeftAzoto)) (Components|Activation|IsActive (Variables|Default|GetRightAzoto)))
    (bind _asthird_person_character (Utilities|Casting|CastToThirdPersonCharacter OtherActor))
    (Default|Muori _asthird_person_character "NewEnumerator0")))

(event EventTick
  (params (DeltaSeconds :type Float%20%28single-precision%29))
  (if (Variables|Default|GetEnabled)
    (Utilities|FlowControl|Delay 4.0)
    (Components|Activation|Activate (Variables|Default|GetLeftAzoto) true)
    (Components|Activation|Activate (Variables|Default|GetRightAzoto) true)
    (Utilities|FlowControl|Delay (Variables|Default|GetFrequency))
    (Components|Activation|Deactivate (Variables|Default|GetLeftAzoto))
    (Components|Activation|Deactivate (Variables|Default|GetRightAzoto))))

(fn ConstructionScript)