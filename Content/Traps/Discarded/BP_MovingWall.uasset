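; BP_MovingWall is a trap wall that slides forward and shoves the player along with it.
; A MoveForward timeline offsets the Wall on local X by its track value plus Speed, destroying the actor once accumulated Speed reaches MaxDistance.
; Any overlap on Frontal opens a Tick gate that teleports player 0 along the actor's forward vector by a fixed step until overlap ends.
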(event OnComponentBeginOverlap(Frontal)
  (params (OverlappedComponent :type Primitive%20Component%20Object%20Reference) (OtherActor :type Actor%20Object%20Reference) (OtherComp :type Primitive%20Component%20Object%20Reference) (OtherBodyIndex :type Integer) (bFromSweep :type Boolean) (SweepResult :type Hit%20Result%20Structure%20%28by%20ref%29))
  (Utilities|FlowControl|Gate true) ; enters at Open
)

(event OnComponentEndOverlap(Frontal)
  (params (OverlappedComponent :type Primitive%20Component%20Object%20Reference) (OtherActor :type Actor%20Object%20Reference) (OtherComp :type Primitive%20Component%20Object%20Reference) (OtherBodyIndex :type Integer))
  (Utilities|FlowControl|Gate true) ; enters at Close
)

(event EventBeginPlay
  (bind _forward (Timeline|MoveForward Play)
    (:Update
      (Transformation|AddLocalOffset (Variables|Default|GetWall) (Math|Vector|MakeVector (+ _forward (Variables|Default|GetSpeed)) 0.0 0.0) false false)
      (Variables|Default|SetDistanceMoved (+ (Variables|Default|GetSpeed) (Variables|Default|GetDistanceMoved)))
      (if (>= (+ (Variables|Default|GetSpeed) (Variables|Default|GetDistanceMoved)) (Variables|Default|GetMaxDistance))
        (Actor|DestroyActor)
        (Timeline|MoveForward Stop)))))

(event EventTick
  (params (DeltaSeconds :type Float%20%28single-precision%29))
  (Utilities|FlowControl|Gate true
    (:Exit
      (Transformation|AddActorWorldOffset (Game|Player|GetPlayerPawn 0) (* (Math|Vector|GetForwardVector (Transformation|GetActorRotation self)) 2.0) false true))))

(fn ConstructionScript)