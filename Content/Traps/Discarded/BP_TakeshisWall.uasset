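; Trap spawner that periodically sends out pairs of moving walls across three lanes, leaving one random lane open.
; A looping timer started on BeginPlay calls SpawnWalls, which, while Active, randomly picks two of the center and side positions.
; Each spawned BP_MovingWall receives the configured speed and travel distance.
; Side lanes are offset along world Y by wall width plus a fixed gap, regardless of the spawner's rotation.
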(event EventBeginPlay
  (Utilities|Time|SetTimerbyFunctionName 0 "SpawnWalls" (Variables|Default|GetWallsFrequency) true))

(fn ConstructionScript)

(fn SpawnWalls
  (bind _self self)
  (bind _self_2 self)
  (bind _self_3 self)
  (bind _defaultsceneroot (Variables|Default|GetDefaultSceneRoot _self))
  (bind _defaultsceneroot_2 (Variables|Default|GetDefaultSceneRoot _self_2))
  (bind _defaultsceneroot_3 (Variables|Default|GetDefaultSceneRoot _self_3))
  (bind _returnvalue (Transformation|GetWorldTransform _defaultsceneroot))
  (bind _returnvalue_2 (Transformation|GetWorldTransform _defaultsceneroot_2))
  (bind _returnvalue_3 (Transformation|GetWorldTransform _defaultsceneroot_3))
  (if (Variables|Default|GetActive)
    (switch int (Math|Random|RandomInteger 3)
      (:0
        (Utilities|FlowControl|Sequence
          (:then_0
            (bind _returnvalue_4 (Game|SpawnActorfromClass (Variables|Default|GetWallType) (Math|Transform|MakeTransform (Math|Vector|MakeVector (.x (.location _returnvalue_2)) (.y (.location _returnvalue_2)) (+ (.z (.location _returnvalue_2)) (/ (Variables|Default|GetWallHeigth) 2.0))) (.rotation _returnvalue_2) (.scale _returnvalue_2)) "Undefined" 0 0 :!label _label))
            (bind _asbp_moving_wall (Utilities|Casting|CastToBP_MovingWall _returnvalue_4))
            (Variables|/Game/Traps/Discarded/BP_MovingWall.BP_MovingWall_C|SetSpeed _asbp_moving_wall (Variables|Default|GetWallsSpeed))
            (Variables|/Game/Traps/Discarded/BP_MovingWall.BP_MovingWall_C|SetMaxDistance _asbp_moving_wall (Variables|Default|GetDistanceToMove)))
          (:then_1
            (bind _returnvalue_5 (Game|SpawnActorfromClass (Variables|Default|GetWallType) (Math|Transform|MakeTransform (Math|Vector|MakeVector (.x (.location _returnvalue)) (- (- (.y (.location _returnvalue)) (Variables|Default|GetWallWidth)) 15.0) (+ (.z (.location _returnvalue)) (/ (Variables|Default|GetWallHeigth) 2.0))) (.rotation _returnvalue) (.scale _returnvalue)) "Undefined" 0 0 :!label _label_2))
            (bind _asbp_moving_wall_2 (Utilities|Casting|CastToBP_MovingWall _returnvalue_5))
            (Variables|/Game/Traps/Discarded/BP_MovingWall.BP_MovingWall_C|SetSpeed _asbp_moving_wall_2 (Variables|Default|GetWallsSpeed))
            (Variables|/Game/Traps/Discarded/BP_MovingWall.BP_MovingWall_C|SetMaxDistance _asbp_moving_wall_2 (Variables|Default|GetDistanceToMove)))))
      (:1
        (Utilities|FlowControl|Sequence
          (:then_0
            (bind _returnvalue_6 (Game|SpawnActorfromClass (Variables|Default|GetWallType) (Math|Transform|MakeTransform (Math|Vector|MakeVector (.x (.location _returnvalue_3)) (+ (+ (.y (.location _returnvalue_3)) (Variables|Default|GetWallWidth)) 15.0) (+ (.z (.location _returnvalue_3)) (/ (Variables|Default|GetWallHeigth) 2.0))) (.rotation _returnvalue_3) (.scale _returnvalue_3)) "Undefined" 0 0 :!label _label_3))
            (bind _asbp_moving_wall_3 (Utilities|Casting|CastToBP_MovingWall _returnvalue_6))
            (Variables|/Game/Traps/Discarded/BP_MovingWall.BP_MovingWall_C|SetSpeed _asbp_moving_wall_3 (Variables|Default|GetWallsSpeed))
            (Variables|/Game/Traps/Discarded/BP_MovingWall.BP_MovingWall_C|SetMaxDistance _asbp_moving_wall_3 (Variables|Default|GetDistanceToMove)))
          (:then_1
            (goto _label_2))))
      (:2
        (Utilities|FlowControl|Sequence
          (:then_0
            (goto _label_3))
          (:then_1
            (goto _label)))))))

(fn Empty)