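; Trap tunnel with doors at both ends that secretly relocates itself, along with the player, to a second point.
; Each door's collision volume plays or reverses a timeline that sets the door's absolute world Z when the character enters or leaves.
; On first overlap with ExitTeleport, the whole actor teleports to SecondPoint with zero rotation, then moves the player to the trigger's new X/Y, keeping height and facing.
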(event OnComponentBeginOverlap(ExitDoorCollision)
  (params (OverlappedComponent :type Primitive%20Component%20Object%20Reference) (OtherActor :type Actor%20Object%20Reference) (OtherComp :type Primitive%20Component%20Object%20Reference) (OtherBodyIndex :type Integer) (bFromSweep :type Boolean) (SweepResult :type Hit%20Result%20Structure%20%28by%20ref%29))
  (bind _exitdoor (Variables|Default|GetExitDoor))
  (bind _returnvalue (Transformation|GetWorldLocation _exitdoor))
  ;[1 1 1] Manage End Tunnel Door
  (Utilities|Casting|CastToThirdPersonCharacter OtherActor)
  (bind _newtrack_1 (Timeline|Timeline_1 Play)
    (:Update
      (Transformation|SetWorldLocation _exitdoor (Math|Vector|MakeVector (.x _returnvalue) (.y _returnvalue) (.z _newtrack_1)) false false))))

(event OnComponentEndOverlap(ExitDoorCollision)
  (params (OverlappedComponent :type Primitive%20Component%20Object%20Reference) (OtherActor :type Actor%20Object%20Reference) (OtherComp :type Primitive%20Component%20Object%20Reference) (OtherBodyIndex :type Integer))
  (bind _exitdoor (Variables|Default|GetExitDoor))
  (bind _returnvalue (Transformation|GetWorldLocation _exitdoor))
  ;[1 1 1] Manage End Tunnel Door
  (Utilities|Casting|CastToThirdPersonCharacter OtherActor)
  (bind _newtrack_1 (Timeline|Timeline_1 Reverse)
    (:Update
      (Transformation|SetWorldLocation _exitdoor (Math|Vector|MakeVector (.x _returnvalue) (.y _returnvalue) (.z _newtrack_1)) false false))))

(event OnComponentBeginOverlap(EnterDoorCollision)
  (params (OverlappedComponent :type Primitive%20Component%20Object%20Reference) (OtherActor :type Actor%20Object%20Reference) (OtherComp :type Primitive%20Component%20Object%20Reference) (OtherBodyIndex :type Integer) (bFromSweep :type Boolean) (SweepResult :type Hit%20Result%20Structure%20%28by%20ref%29))
  (bind _entrydoor (Variables|Default|GetEntryDoor))
  (bind _returnvalue (Transformation|GetWorldLocation _entrydoor))
  ;[1 1 1] Manage Tunnel door
  (Utilities|Casting|CastToThirdPersonCharacter OtherActor)
  (bind _newtrack_1 (Timeline|Timeline_0 Play)
    (:Update
      (Transformation|SetWorldLocation _entrydoor (Math|Vector|MakeVector (.x _returnvalue) (.y _returnvalue) (.z _newtrack_1)) false false))))

(event OnComponentEndOverlap(EnterDoorCollision)
  (params (OverlappedComponent :type Primitive%20Component%20Object%20Reference) (OtherActor :type Actor%20Object%20Reference) (OtherComp :type Primitive%20Component%20Object%20Reference) (OtherBodyIndex :type Integer))
  (bind _entrydoor (Variables|Default|GetEntryDoor))
  (bind _returnvalue (Transformation|GetWorldLocation _entrydoor))
  ;[1 1 1] Manage Tunnel door
  (Utilities|Casting|CastToThirdPersonCharacter OtherActor)
  (bind _newtrack_1 (Timeline|Timeline_0 Reverse)
    (:Update
      (Transformation|SetWorldLocation _entrydoor (Math|Vector|MakeVector (.x _returnvalue) (.y _returnvalue) (.z _newtrack_1)) false false))))

(event OnComponentBeginOverlap(ExitTeleport)
  (params (OverlappedComponent :type Primitive%20Component%20Object%20Reference) (OtherActor :type Actor%20Object%20Reference) (OtherComp :type Primitive%20Component%20Object%20Reference) (OtherBodyIndex :type Integer) (bFromSweep :type Boolean) (SweepResult :type Hit%20Result%20Structure%20%28by%20ref%29))
  (bind _returnvalue (Game|Player|GetPlayerPawn 0))
  (bind _exitteleport (Variables|Default|GetExitTeleport))
  (bind _returnvalue_2 (Transformation|GetWorldLocation _exitteleport))
  (bind _returnvalue_3 (Transformation|GetActorLocation _returnvalue))
  (Utilities|Casting|CastToThirdPersonCharacter OtherActor)
  (if (not (Variables|Default|GetTeleported))
    (Transformation|Teleport (Transformation|GetActorLocation (Variables|Default|GetSecondPoint)) "0, 0, 0")
    (Variables|Default|SetTeleported true)
    (Transformation|Teleport _returnvalue (Math|Vector|MakeVector (+ (.x _returnvalue_3) (- (.x _returnvalue_2) (.x _returnvalue_3))) (+ (- (.y _returnvalue_2) (.y _returnvalue_3)) (.y _returnvalue_3)) (.z _returnvalue_3)) (Transformation|GetActorRotation _returnvalue))))

(fn ConstructionScript)